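; BP_BoardManager is a chess board manager actor that, as it stands, only caches the BP_ChessGameState on BeginPlay and prints if the cast fails.
; CheckAvailable and CheckPieceMoves are stubs, the latter always returning InCheck as false.
; Disconnected graphs hold unused board builders that lay out an 8x8 checkered grid from index division and modulo, either as spawned, numbered BP_Tile actors or construction-script mesh components.
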(event EventBeginPlay
  (Utilities|FlowControl|Sequence
    (:then_0
      (bind _asbp_chess_game_state (Utilities|Casting|CastToBP_ChessGameState (Game|GetGameState))
        (:then
          (Variables|Default|SetAs%20Chess%20Game%20State _asbp_chess_game_state))
        (:CastFailed
          (Development|PrintString "Hello" true true "(R=1.000000,G=0.000000,B=0.039492,A=1.000000)" 7.0))))))

(event Collision|EventActorBeginOverlap
  (params (OtherActor :type Actor%20Object%20Reference)))

(event EventTick
  (params (DeltaSeconds :type Float%20%28single-precision%29)))

(fn ConstructionScript)

(fn CheckAvailable
  (params (Tiles :type Array%20of%20BP%20Tile%20Object%20References))
  (return 0))

(fn CheckPieceMoves
  (return 0 0 false 0 0))