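; BP_King is the king piece in a multiplayer chess template, handling movement, castling and check detection.
; It caches enemy pieces after a startup delay, using their moves to filter unsafe adjacent tiles and record attackers.
; MovePiece validates through PieceMoveLogic, destroys captured pieces, moves via SvrPieceMove and triggers the rook's castling.
; CheckAvailable lists legal destinations using tile-number offsets, with castling mirrored per team; CheckMoves is a stub.
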(event EventBeginPlay
  (|CallParentFunction)
  (Utilities|FlowControl|Delay 2.0)
  (bind _outactors (Actor|GetAllActorsOfClass "/Game/MPChessTemplate/Blueprints/BP_ChessPieces.BP_ChessPieces_C"))
  (for _array_element _outactors
    (if (!= (Variables|/Game/MPChessTemplate/Blueprints/BP_ChessPieces.BP_ChessPieces_C|GetTeam _array_element) (Variables|Default|GetTeam))
      (Utilities|Array|Add (Variables|Default|GetEnemyPieces) _array_element))))

(event Collision|EventActorBeginOverlap
  (params (OtherActor :type Actor%20Object%20Reference))
  (|CallParentFunction OtherActor) ; This node is disabled and will not be called.\nDrag off pins to build functionality.
)

(event EventTick
  (params (DeltaSeconds :type Float%20%28single-precision%29))
  (|CallParentFunction DeltaSeconds) ; This node is disabled and will not be called.\nDrag off pins to build functionality.
)

(event EventMovePiece
  (params (Piece :type BP%20Chess%20Pieces%20Object%20Reference) (Tile :type BP%20Tile%20Object%20Reference) (Number :type Integer) (Location :type Vector :default "0, 0, 0"))
  (if (not (Variables|/Game/MPChessTemplate/Blueprints/BP_Tile.BP_Tile_C|GetKing? Tile))
    (Variables|Default|SetRookTile 0)
    (Variables|Default|SetRook 0)
    (bind _array_element (Utilities|Array|ForEachLoopwithBreak (Variables|Default|GetOut%20Actors) :!label _label)
      (:LoopBody
        (if (== (Variables|Default|GetCurrentTile) (Variables|/Game/MPChessTemplate/Blueprints/BP_Tile.BP_Tile_C|GetTileNumber _array_element))
          (Variables|/Game/MPChessTemplate/Blueprints/BP_Tile.BP_Tile_C|SetPiece _array_element 0)
          (Variables|Default|SetLastTile _array_element)
          (goto _label Break)))
      (:Completed
        (bind (_valid _take) (CallFunction|PieceMoveLogic Number (Variables|/Game/MPChessTemplate/Blueprints/BP_Tile.BP_Tile_C|GetOccupied Tile) (Variables|Default|GetFirstMove?) (and (Variables|/Game/MPChessTemplate/Blueprints/BP_Tile.BP_Tile_C|GetOccupied Tile) (!= (Variables|Default|GetTeam) (Variables|/Game/MPChessTemplate/Blueprints/BP_Tile.BP_Tile_C|GetTeam Tile))) false))
        (if _valid
          (if (Variables|/Game/MPChessTemplate/Blueprints/BP_Tile.BP_Tile_C|GetOccupied Tile)
            (if (!= (Variables|/Game/MPChessTemplate/Blueprints/BP_Tile.BP_Tile_C|GetTeam Tile) (Variables|Default|GetTeam))
              (bind _piece (Variables|/Game/MPChessTemplate/Blueprints/BP_Tile.BP_Tile_C|GetPiece Tile)
                (:then
                  (Default|DestroyPiece _piece))
                (:else
                  _))
              (CallFunction|SvrPieceMove Number Location Tile :!label _label_2)
              (Variables|Default|SetFirstMove? false)
              (Variables|/Game/MPChessTemplate/Blueprints/BP_Tile.BP_Tile_C|SetPiece Tile self)
              (Variables|/Game/MPChessTemplate/Blueprints/BP_Tile.BP_Tile_C|SetTeam Tile (Variables|Default|GetTeam))
              (Variables|/Game/MPChessTemplate/Blueprints/BP_Tile.BP_Tile_C|SetKing? Tile true)
              (Variables|/Game/MPChessTemplate/Blueprints/BP_Tile.BP_Tile_C|SetOccupied (Variables|Default|GetLastTile) false)
              (Variables|/Game/MPChessTemplate/Blueprints/BP_Tile.BP_Tile_C|SetKing? (Variables|Default|GetLastTile) false)
              ;[1 1 1] Castling
              (if _take
                (bind _array_element_2 (Utilities|Array|ForEachLoopwithBreak (Variables|Default|GetOut%20Actors) :!label _label_3)
                  (:LoopBody
                    (if (== (Variables|Default|GetRookTile) (Variables|/Game/MPChessTemplate/Blueprints/BP_Tile.BP_Tile_C|GetTileNumber _array_element_2))
                      (Default|Castling (Variables|Default|GetRook) _array_element_2 (Transformation|GetActorLocation _array_element_2) (Variables|/Game/MPChessTemplate/Blueprints/BP_Tile.BP_Tile_C|GetTileNumber _array_element_2))
                      (goto _label_3 Break))))))
            (else
              (goto _label_2))))))))

(event EventKinginCheck?
  (Utilities|Array|Clear (Variables|Default|GetInCheckTiles))
  (Utilities|Array|Clear (Variables|Default|GetValidMoves))
  (bind _validmoves (CallFunction|CheckPieceMoves))
  (Variables|Default|SetValidMoves _validmoves))

(event EventDestroyPiece
  (params (Piece :type BP%20Chess%20Pieces%20Object%20Reference))
  (bind _enemypieces (Variables|Default|GetEnemyPieces))
  (bind _array_element (Utilities|Array|ForEachLoopwithBreak _enemypieces :!label _label)
    (:LoopBody
      (if (== _array_element Piece)
        (Utilities|Array|RemoveItem _enemypieces Piece)
        (goto _label Break)))))

(fn ConstructionScript
  (|CallParentFunction))

(fn PieceMoveLogic
  (params (Tile :type Integer) (Occupied? :type Boolean) (FirstMove? :type Boolean) (EnemyOccupied? :type Boolean) (KingInCheck? :type Boolean))
  (bind _currenttile (Variables|Default|GetCurrentTile))
  (bind _out_actors (Variables|Default|GetOut%20Actors))
  (bind _availablility (LocalVariables|GetAvailablility))
  (bind _out_actors_2 (Variables|Default|GetOut%20Actors))
  (Utilities|Array|Clear (LocalVariables|GetLeftCastleSlots))
  (Utilities|Array|Clear (LocalVariables|GetRighCastleSlots))
  (if (Utilities|Array|ContainsItem (Variables|Default|GetStepUnit) (Math|Integer|Absolute(Integer) (- Tile (Variables|Default|GetCurrentTile))))
    (for _array_element (Variables|Default|GetEnemyPieces)
      (if (Utilities|Array|ContainsItem (Variables|/Game/MPChessTemplate/Blueprints/BP_ChessPieces.BP_ChessPieces_C|GetValidMoves _array_element) Tile)
        (Utilities|Array|AddUnique _availablility true)
        (else
          (Utilities|Array|AddUnique _availablility false))))
    (if (Utilities|Array|ContainsItem (LocalVariables|GetAvailablility) true)
      (return false false)
      (else
        (return true false)))
    (elif (== Tile (+ _currenttile 2))
      (if (Variables|Default|GetFirstMove?)
        (switch int (Variables|Default|GetTeam)
          (:1
            ;[1 1 1] Team White Castling
            ;;[1 1 1] Check Tiles (Right-SideCastling)
            (for _array_element_2 (LocalVariables|GetCastlingSlots)
              (bind _array_element_3 (Utilities|Array|ForEachLoopwithBreak _out_actors :!label _label)
                (:LoopBody
                  (if (== (Variables|/Game/MPChessTemplate/Blueprints/BP_Tile.BP_Tile_C|GetTileNumber _array_element_3) (+ _array_element_2 (Variables|Default|GetCurrentTile)))
                    (Utilities|Array|AddUnique (LocalVariables|GetRighCastleSlots) (Variables|/Game/MPChessTemplate/Blueprints/BP_Tile.BP_Tile_C|GetOccupied _array_element_3))
                    (goto _label Break)))))
            (if (Utilities|Array|ContainsItem (LocalVariables|GetRighCastleSlots) true)
              (return false false)
              (else
                ;;[1 1 1] Right
                (bind _array_element_4 (Utilities|Array|ForEachLoopwithBreak _out_actors :!label _label_2)
                  (:LoopBody
                    (if (== (Variables|/Game/MPChessTemplate/Blueprints/BP_Tile.BP_Tile_C|GetTileNumber _array_element_4) (+ (Variables|Default|GetCurrentTile) 3))
                      (if (and (== (Utilities|GetClass (Variables|/Game/MPChessTemplate/Blueprints/BP_Tile.BP_Tile_C|GetPiece _array_element_4)) "/Game/MPChessTemplate/Blueprints/BP_Rooks.BP_Rooks_C") (Variables|/Game/MPChessTemplate/Blueprints/BP_ChessPieces.BP_ChessPieces_C|GetFirstMove? (Variables|/Game/MPChessTemplate/Blueprints/BP_Tile.BP_Tile_C|GetPiece _array_element_4)))
                        (Utilities|FlowControl|Sequence
                          (:then_0
                            (Variables|Default|SetRook (Variables|/Game/MPChessTemplate/Blueprints/BP_Tile.BP_Tile_C|GetPiece _array_element_4))
                            (Variables|Default|SetRookTile (+ (Variables|Default|GetCurrentTile) 1))
                            (return true true))
                          (:then_1
                            (goto _label_2 Break)))
                        (else
                          (return false false)))))))))
          (:2
            ;[1 1 1] Team Black Castling
            ;;[1 1 1] Check Tiles (Right-SideCastling)
            (for _array_element_5 (LocalVariables|GetCastlingSlots)
              (bind _array_element_6 (Utilities|Array|ForEachLoopwithBreak _out_actors_2 :!label _label_3)
                (:LoopBody
                  (if (== (Variables|/Game/MPChessTemplate/Blueprints/BP_Tile.BP_Tile_C|GetTileNumber _array_element_6) (- (Variables|Default|GetCurrentTile) _array_element_5))
                    (Utilities|Array|AddUnique (LocalVariables|GetRighCastleSlots) (Variables|/Game/MPChessTemplate/Blueprints/BP_Tile.BP_Tile_C|GetOccupied _array_element_6))
                    (goto _label_3 Break)))))
            (if (Utilities|Array|ContainsItem (LocalVariables|GetRighCastleSlots) true)
              (return false false)
              (else
                ;;[1 1 1] Right
                (bind _array_element_7 (Utilities|Array|ForEachLoopwithBreak _out_actors_2 :!label _label_4)
                  (:LoopBody
                    (if (== (Variables|/Game/MPChessTemplate/Blueprints/BP_Tile.BP_Tile_C|GetTileNumber _array_element_7) (- (Variables|Default|GetCurrentTile) 3))
                      (if (and (== (Utilities|GetClass (Variables|/Game/MPChessTemplate/Blueprints/BP_Tile.BP_Tile_C|GetPiece _array_element_7)) "/Game/MPChessTemplate/Blueprints/BP_Rooks.BP_Rooks_C") (Variables|/Game/MPChessTemplate/Blueprints/BP_ChessPieces.BP_ChessPieces_C|GetFirstMove? (Variables|/Game/MPChessTemplate/Blueprints/BP_Tile.BP_Tile_C|GetPiece _array_element_7)))
                        (Utilities|FlowControl|Sequence
                          (:then_0
                            (goto _label_4 Break))
                          (:then_1
                            (Variables|Default|SetRook (Variables|/Game/MPChessTemplate/Blueprints/BP_Tile.BP_Tile_C|GetPiece _array_element_7))
                            (Variables|Default|SetRookTile (- (Variables|Default|GetCurrentTile) 1))
                            (return true true)))
                        (else
                          (return false false))))))))))
        (else
          (return false false)))
      (elif (== Tile (- _currenttile 2))
        (switch int (Variables|Default|GetTeam)
          (:1
            ;;[1 1 1] CheckTiles (Left Side Castling)
            (for _array_element_8 (LocalVariables|GetCastlingSlots2)
              (bind _array_element_9 (Utilities|Array|ForEachLoopwithBreak _out_actors :!label _label_5)
                (:LoopBody
                  (if (== (Variables|/Game/MPChessTemplate/Blueprints/BP_Tile.BP_Tile_C|GetTileNumber _array_element_9) (- (Variables|Default|GetCurrentTile) _array_element_8))
                    (Utilities|Array|AddUnique (LocalVariables|GetLeftCastleSlots) (Variables|/Game/MPChessTemplate/Blueprints/BP_Tile.BP_Tile_C|GetOccupied _array_element_9))
                    (goto _label_5 Break)))))
            (if (Utilities|Array|ContainsItem (LocalVariables|GetLeftCastleSlots) true)
              (return false false)
              (else
                ;;[1 1 1] Left
                (bind _array_element_10 (Utilities|Array|ForEachLoopwithBreak (Variables|Default|GetOut%20Actors) :!label _label_6)
                  (:LoopBody
                    (if (== (Variables|/Game/MPChessTemplate/Blueprints/BP_Tile.BP_Tile_C|GetTileNumber _array_element_10) (- (Variables|Default|GetCurrentTile) 4))
                      (if (and (== (Utilities|GetClass (Variables|/Game/MPChessTemplate/Blueprints/BP_Tile.BP_Tile_C|GetPiece _array_element_10)) "/Game/MPChessTemplate/Blueprints/BP_Rooks.BP_Rooks_C") (Variables|/Game/MPChessTemplate/Blueprints/BP_ChessPieces.BP_ChessPieces_C|GetFirstMove? (Variables|/Game/MPChessTemplate/Blueprints/BP_Tile.BP_Tile_C|GetPiece _array_element_10)))
                        (Utilities|FlowControl|Sequence
                          (:then_0
                            (goto _label_6 Break))
                          (:then_1
                            (Variables|Default|SetRook (Variables|/Game/MPChessTemplate/Blueprints/BP_Tile.BP_Tile_C|GetPiece _array_element_10))
                            (Variables|Default|SetRookTile (+ (Variables|Default|GetCurrentTile) 1))
                            (return true true)))
                        (else
                          (return false false)))))))))
          (:2
            ;;[1 1 1] CheckTiles (Left Side Castling)
            (for _array_element_11 (LocalVariables|GetCastlingSlots2)
              (bind _array_element_12 (Utilities|Array|ForEachLoopwithBreak _out_actors_2 :!label _label_7)
                (:LoopBody
                  (if (== (Variables|/Game/MPChessTemplate/Blueprints/BP_Tile.BP_Tile_C|GetTileNumber _array_element_12) (+ (Variables|Default|GetCurrentTile) _array_element_11))
                    (Utilities|Array|AddUnique (LocalVariables|GetLeftCastleSlots) (Variables|/Game/MPChessTemplate/Blueprints/BP_Tile.BP_Tile_C|GetOccupied _array_element_12))
                    (goto _label_7 Break)))))
            (if (Utilities|Array|ContainsItem (LocalVariables|GetLeftCastleSlots) true)
              (return false false)
              (else
                ;;[1 1 1] Left
                (bind _array_element_13 (Utilities|Array|ForEachLoopwithBreak (Variables|Default|GetOut%20Actors) :!label _label_8)
                  (:LoopBody
                    (if (== (Variables|/Game/MPChessTemplate/Blueprints/BP_Tile.BP_Tile_C|GetTileNumber _array_element_13) (+ (Variables|Default|GetCurrentTile) 4))
                      (if (and (== (Utilities|GetClass (Variables|/Game/MPChessTemplate/Blueprints/BP_Tile.BP_Tile_C|GetPiece _array_element_13)) "/Game/MPChessTemplate/Blueprints/BP_Rooks.BP_Rooks_C") (Variables|/Game/MPChessTemplate/Blueprints/BP_ChessPieces.BP_ChessPieces_C|GetFirstMove? (Variables|/Game/MPChessTemplate/Blueprints/BP_Tile.BP_Tile_C|GetPiece _array_element_13)))
                        (Utilities|FlowControl|Sequence
                          (:then_0
                            (goto _label_8 Break))
                          (:then_1
                            (Variables|Default|SetRook (Variables|/Game/MPChessTemplate/Blueprints/BP_Tile.BP_Tile_C|GetPiece _array_element_13))
                            (Variables|Default|SetRookTile (- (Variables|Default|GetCurrentTile) 1))
                            (return true true)))
                        (else
                          (return false false))))))))))
        (else
          (return false false))))))

(fn CheckAvailable
  (params (Tiles :type Array%20of%20BP%20Tile%20Object%20References))
  (bind _currenttile (Variables|Default|GetCurrentTile))
  (bind _currenttile_2 (Variables|Default|GetCurrentTile))
  (bind _currenttile_3 (Variables|Default|GetCurrentTile))
  (bind _currenttile_4 (Variables|Default|GetCurrentTile))
  (LocalVariables|SetLeftCastle false)
  (LocalVariables|SetRightCastle false)
  (Utilities|Array|Clear (LocalVariables|GetLeftCastleSlots))
  (Utilities|Array|Clear (LocalVariables|GetRighCastleSlots))
  (if (Variables|Default|GetFirstMove?)
    ;[1 1 1] Check Team
    (switch int (Variables|Default|GetTeam)
      (:1
        ;[1 1 1] Team White Castling
        ;;[1 1 1] Check Tiles (Right-SideCastling)
        (for _array_element (LocalVariables|GetCastlingSlots)
          (bind _array_element_2 (Utilities|Array|ForEachLoopwithBreak Tiles :!label _label)
            (:LoopBody
              (if (== (Variables|/Game/MPChessTemplate/Blueprints/BP_Tile.BP_Tile_C|GetTileNumber _array_element_2) (+ _array_element (Variables|Default|GetCurrentTile)))
                (Utilities|Array|AddUnique (LocalVariables|GetRighCastleSlots) (Variables|/Game/MPChessTemplate/Blueprints/BP_Tile.BP_Tile_C|GetOccupied _array_element_2))
                (goto _label Break)))))
        (if (Utilities|Array|ContainsItem (LocalVariables|GetRighCastleSlots) true)
          ;;[1 1 1] CheckTiles (Left Side Castling)
          (for _array_element_3 (LocalVariables|GetCastlingSlots2) :!label _label_2
            (bind _array_element_4 (Utilities|Array|ForEachLoopwithBreak Tiles :!label _label_3)
              (:LoopBody
                (if (== (Variables|/Game/MPChessTemplate/Blueprints/BP_Tile.BP_Tile_C|GetTileNumber _array_element_4) (- (Variables|Default|GetCurrentTile) _array_element_3))
                  (Utilities|Array|AddUnique (LocalVariables|GetLeftCastleSlots) (Variables|/Game/MPChessTemplate/Blueprints/BP_Tile.BP_Tile_C|GetOccupied _array_element_4))
                  (goto _label_3 Break)))))
          (if (Utilities|Array|ContainsItem (LocalVariables|GetLeftCastleSlots) true)
            ;[1 1 1] 1-tile moves (All Directions)
            (for _array_element_5 (Variables|Default|GetStepUnit) :!label _label_4
              (for _array_element_6 Tiles
                (if (== (Variables|/Game/MPChessTemplate/Blueprints/BP_Tile.BP_Tile_C|GetTileNumber _array_element_6) (+ (Variables|Default|GetCurrentTile) _array_element_5))
                  (if (Variables|/Game/MPChessTemplate/Blueprints/BP_Tile.BP_Tile_C|GetOccupied _array_element_6)
                    (if (!= (Variables|/Game/MPChessTemplate/Blueprints/BP_Tile.BP_Tile_C|GetTeam _array_element_6) (Variables|Default|GetTeam))
                      (Utilities|Array|AddUnique (LocalVariables|GetLocalValidMoves) (+ (Variables|Default|GetCurrentTile) _array_element_5) :!label _label_5))
                    (else
                      (goto _label_5))))))
            ;[1 1 1] Check if dangerous tile
            (for _array_element_7 (Variables|Default|GetEnemyPieces)
              (bind _validmoves (Default|CheckPieceMoves _array_element_7))
              (for _array_element_8 _validmoves
                (Utilities|Array|RemoveItem (LocalVariables|GetLocalValidMoves) _array_element_8)))
            (return (LocalVariables|GetLocalValidMoves))
            (else
              ;;[1 1 1] Left
              (bind _array_element_9 (Utilities|Array|ForEachLoopwithBreak Tiles :!label _label_6)
                (:LoopBody
                  (if (== (Variables|/Game/MPChessTemplate/Blueprints/BP_Tile.BP_Tile_C|GetTileNumber _array_element_9) (- _currenttile_4 4))
                    (if (and (== (Utilities|GetClass (Variables|/Game/MPChessTemplate/Blueprints/BP_Tile.BP_Tile_C|GetPiece _array_element_9)) "/Game/MPChessTemplate/Blueprints/BP_Rooks.BP_Rooks_C") (Variables|/Game/MPChessTemplate/Blueprints/BP_ChessPieces.BP_ChessPieces_C|GetFirstMove? (Variables|/Game/MPChessTemplate/Blueprints/BP_Tile.BP_Tile_C|GetPiece _array_element_9)))
                      (LocalVariables|SetLeftCastle true)
                      (goto _label_6 Break))))
                (:Completed
                  (if (LocalVariables|GetLeftCastle)
                    (Utilities|Array|AddUnique (LocalVariables|GetLocalValidMoves) (- _currenttile_4 2))
                    (goto _label_4)
                    (else
                      (goto _label_4)))))))
          (else
            ;;[1 1 1] Right
            (bind _array_element_10 (Utilities|Array|ForEachLoopwithBreak Tiles :!label _label_7)
              (:LoopBody
                (if (== (Variables|/Game/MPChessTemplate/Blueprints/BP_Tile.BP_Tile_C|GetTileNumber _array_element_10) (+ _currenttile_3 3))
                  (if (and (== (Utilities|GetClass (Variables|/Game/MPChessTemplate/Blueprints/BP_Tile.BP_Tile_C|GetPiece _array_element_10)) "/Game/MPChessTemplate/Blueprints/BP_Rooks.BP_Rooks_C") (Variables|/Game/MPChessTemplate/Blueprints/BP_ChessPieces.BP_ChessPieces_C|GetFirstMove? (Variables|/Game/MPChessTemplate/Blueprints/BP_Tile.BP_Tile_C|GetPiece _array_element_10)))
                    (LocalVariables|SetRightCastle true)
                    (goto _label_7 Break)
                    (else
                      (goto _label_2)))))
              (:Completed
                (if (LocalVariables|GetRightCastle)
                  (Utilities|Array|AddUnique (LocalVariables|GetLocalValidMoves) (+ _currenttile_3 2))
                  (goto _label_2)
                  (else
                    (goto _label_2))))))))
      (:2
        ;[1 1 1] Team Blacl Castling
        ;;[1 1 1] Check Tiles (Right-SideCastling)
        (for _array_element_11 (LocalVariables|GetCastlingSlots)
          (bind _array_element_12 (Utilities|Array|ForEachLoopwithBreak Tiles :!label _label_8)
            (:LoopBody
              (if (== (Variables|/Game/MPChessTemplate/Blueprints/BP_Tile.BP_Tile_C|GetTileNumber _array_element_12) (- (Variables|Default|GetCurrentTile) _array_element_11))
                (Utilities|Array|AddUnique (LocalVariables|GetRighCastleSlots) (Variables|/Game/MPChessTemplate/Blueprints/BP_Tile.BP_Tile_C|GetOccupied _array_element_12))
                (goto _label_8 Break)))))
        (if (Utilities|Array|ContainsItem (LocalVariables|GetRighCastleSlots) true)
          ;;[1 1 1] CheckTiles (Left Side Castling)
          (for _array_element_13 (LocalVariables|GetCastlingSlots2) :!label _label_9
            (bind _array_element_14 (Utilities|Array|ForEachLoopwithBreak Tiles :!label _label_10)
              (:LoopBody
                (if (== (Variables|/Game/MPChessTemplate/Blueprints/BP_Tile.BP_Tile_C|GetTileNumber _array_element_14) (+ (Variables|Default|GetCurrentTile) _array_element_13))
                  (Utilities|Array|AddUnique (LocalVariables|GetLeftCastleSlots) (Variables|/Game/MPChessTemplate/Blueprints/BP_Tile.BP_Tile_C|GetOccupied _array_element_14))
                  (goto _label_10 Break)))))
          (if (Utilities|Array|ContainsItem (LocalVariables|GetLeftCastleSlots) true)
            (goto _label_4)
            (else
              ;;[1 1 1] Left
              (bind _array_element_15 (Utilities|Array|ForEachLoopwithBreak Tiles :!label _label_11)
                (:LoopBody
                  (if (== (Variables|/Game/MPChessTemplate/Blueprints/BP_Tile.BP_Tile_C|GetTileNumber _array_element_15) (+ _currenttile 4))
                    (if (and (== (Utilities|GetClass (Variables|/Game/MPChessTemplate/Blueprints/BP_Tile.BP_Tile_C|GetPiece _array_element_15)) "/Game/MPChessTemplate/Blueprints/BP_Rooks.BP_Rooks_C") (Variables|/Game/MPChessTemplate/Blueprints/BP_ChessPieces.BP_ChessPieces_C|GetFirstMove? (Variables|/Game/MPChessTemplate/Blueprints/BP_Tile.BP_Tile_C|GetPiece _array_element_15)))
                      (LocalVariables|SetLeftCastle true)
                      (goto _label_11 Break))))
                (:Completed
                  (if (LocalVariables|GetLeftCastle)
                    (Utilities|Array|AddUnique (LocalVariables|GetLocalValidMoves) (+ _currenttile 2))
                    (goto _label_4)
                    (else
                      (goto _label_4)))))))
          (else
            ;;[1 1 1] Right
            (bind _array_element_16 (Utilities|Array|ForEachLoopwithBreak Tiles :!label _label_12)
              (:LoopBody
                (if (== (Variables|/Game/MPChessTemplate/Blueprints/BP_Tile.BP_Tile_C|GetTileNumber _array_element_16) (- _currenttile_2 3))
                  (if (and (== (Utilities|GetClass (Variables|/Game/MPChessTemplate/Blueprints/BP_Tile.BP_Tile_C|GetPiece _array_element_16)) "/Game/MPChessTemplate/Blueprints/BP_Rooks.BP_Rooks_C") (Variables|/Game/MPChessTemplate/Blueprints/BP_ChessPieces.BP_ChessPieces_C|GetFirstMove? (Variables|/Game/MPChessTemplate/Blueprints/BP_Tile.BP_Tile_C|GetPiece _array_element_16)))
                    (LocalVariables|SetRightCastle true)
                    (goto _label_12 Break)
                    (else
                      (goto _label_9)))))
              (:Completed
                (if (LocalVariables|GetRightCastle)
                  (Utilities|Array|AddUnique (LocalVariables|GetLocalValidMoves) (- _currenttile_2 2))
                  (goto _label_9)
                  (else
                    (goto _label_9)))))))))
    (else
      (goto _label_4))))

(fn CheckMoves
  (params (Tiles :type Array%20of%20BP%20Tile%20Object%20References))
  (return 0 false 0))

(fn CheckPieceMoves
  (Utilities|Array|Clear (LocalVariables|GetAtkPieces))
  (for _array_element (Variables|Default|GetStepUnit)
    ;[1 1 1] 1-tile moves (All Directions)
    (for _array_element_2 (Variables|Default|GetOut%20Actors)
      (if (== (Variables|/Game/MPChessTemplate/Blueprints/BP_Tile.BP_Tile_C|GetTileNumber _array_element_2) (+ (Variables|Default|GetCurrentTile) _array_element))
        (if (Variables|/Game/MPChessTemplate/Blueprints/BP_Tile.BP_Tile_C|GetOccupied _array_element_2)
          (if (!= (Variables|/Game/MPChessTemplate/Blueprints/BP_Tile.BP_Tile_C|GetTeam _array_element_2) (Variables|Default|GetTeam))
            (Utilities|Array|AddUnique (Variables|Default|GetValidMoves) (+ (Variables|Default|GetCurrentTile) _array_element) :!label _label))
          (else
            (goto _label))))))
  (for _array_element_3 (Variables|Default|GetEnemyPieces)
    (Utilities|IsValid _array_element_3
      (:Is%20Valid
        (for _array_element_4 (Variables|/Game/MPChessTemplate/Blueprints/BP_ChessPieces.BP_ChessPieces_C|GetValidMoves _array_element_3)
          (Utilities|Array|RemoveItem (Variables|Default|GetValidMoves) _array_element_4)
          (if (Utilities|Array|ContainsItem (Variables|/Game/MPChessTemplate/Blueprints/BP_ChessPieces.BP_ChessPieces_C|GetValidMoves _array_element_3) (Variables|Default|GetCurrentTile))
            (LocalVariables|SetChecked true))
          (if (LocalVariables|GetChecked)
            (Utilities|Array|AddUnique (LocalVariables|GetAtkPieces) _array_element_3))))))
  (return (Variables|Default|GetValidMoves) 0 (LocalVariables|GetChecked) 0 (LocalVariables|GetAtkPieces)))