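; BP_ChessGameMode is the game mode for a multiplayer chess match, handling player setup and match start.
; PostLogin hands each controller the next camera transform from StartPoints, then starts the match and calls MatchBegin on the game state once more than one player is present.
; HandleStartingNewPlayer links each controller to its player state and assigns both an incrementing team number.
; A Destroy event provides server-side actor destruction.
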(event Custom|Destroy
  (params (Target :type Actor%20Object%20Reference))
  ;[0.15 0.15 0.15 0.5] Server's Actor Destroying
  (Actor|DestroyActor Target))

(event EventBeginPlay
  (bind _aschess_game_state (Utilities|Casting|CastToBP_ChessGameState (Game|GetGameState)))
  (Variables|Default|SetAs%20Chess%20Game%20State _aschess_game_state))

(event EventHandleStartingNewPlayer
  (params (NewPlayer :type Player%20Controller%20Object%20Reference))
  (bind _newvar (Variables|Default|GetNewVar))
  ;[0.15 0.15 0.15 0.5] Assigns PlayerState class to player
  (bind _aschess_player_state (Utilities|Casting|CastToBP_ChessPlayerState (Variables|/Script/Engine.Controller|GetPlayerState NewPlayer)))
  (bind _aschess_player_controller (Utilities|Casting|CastToBP_ChessPlayerController NewPlayer))
  (Variables|/Game/MPChessTemplate/Blueprints/BP_ChessPlayerController.BP_ChessPlayerController_C|SetAs%20Chess%20Player%20State _aschess_player_controller _aschess_player_state)
  ;[0.15 0.15 0.15 0.5] Assigns Team Number to Player
  (Variables|/Game/MPChessTemplate/Blueprints/BP_ChessPlayerController.BP_ChessPlayerController_C|SetTeam _aschess_player_controller _newvar)
  (Variables|/Game/MPChessTemplate/Blueprints/BP_ChessPlayerState.BP_ChessPlayerState_C|SetTeam _aschess_player_state _newvar)
  (Math|Integer|IncrementInt _newvar))

(event EventPostLogin
  (params (NewPlayer :type Player%20Controller%20Object%20Reference))
  (bind _startpoints (Variables|Default|GetStartPoints))
  ;[0.15 0.15 0.15 0.5] Assigns PlayerController class to player
  (bind _aschess_player_controller (Utilities|Casting|CastToBP_ChessPlayerController NewPlayer))
  ;[0.15 0.15 0.15 0.5] Assigns Camera Position
  (Variables|/Game/MPChessTemplate/Blueprints/BP_ChessPlayerController.BP_ChessPlayerController_C|SetCameraTransform _aschess_player_controller (Utilities|Array|Get(acopy) _startpoints))
  (Utilities|Array|RemoveIndex _startpoints)
  ;[0.15 0.15 0.15 0.5] Check if enough players in session to start match
  (if (> (Class|GameplayStatics|GetNumPlayerStates) 1)
    (Class|GameMode|StartMatch)
    (bind _aschess_game_state (Utilities|Casting|CastToBP_ChessGameState (Game|GetGameState)))
    (Default|MatchBegin _aschess_game_state)))

(fn ConstructionScript)