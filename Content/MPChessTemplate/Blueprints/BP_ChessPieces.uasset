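; Base chess piece Blueprint that handles selection decals, moves, captures and check detection, with stub functions for piece-specific rules.
; MovePiece validates through PieceMoveLogic, destroys any enemy occupant, relocates via SvrPieceMove and updates tile occupancy.
; After a delay it re-evaluates check through CheckPieceMoves, relays the result to the game state and switches turns.
; Captures notify kings and game state before the game mode destroys the piece.
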(event Custom|SvrPieceMove
  (params (Tile :type Integer) (NewLocation :type Vector) (TargetActor :type BP%20Tile%20Object%20Reference))
  ;[1 1 1] Piece Move Execution
  (bind _returnvalue (Transformation|SetActorLocation NewLocation false false))
  (Variables|/Game/MPChessTemplate/Blueprints/BP_Tile.BP_Tile_C|SetOccupied TargetActor _returnvalue)
  (if _returnvalue
    (Variables|Default|SetCurrentTile Tile)))

(event Custom|SvrDestroyPiece
  (params (Target :type Actor%20Object%20Reference))
  (bind _self self)
  (bind _as_chess_game_state (Variables|Default|GetAs%20Chess%20Game%20State))
  ;[1 1 1] Piece Elimanation
  (bind _outactors (Actor|GetAllActorsOfClass "/Game/MPChessTemplate/Blueprints/BP_King.BP_King_C"))
  (for _array_element _outactors
    (Default|DestroyPiece _array_element _self))
  (Utilities|FlowControl|Sequence
    (:then_0
      (Default|DestroyPiece _as_chess_game_state _self)
      (Default|Destroy (Variables|Default|GetAs%20Chess%20Game%20Mode) Target))
    (:then_1
      (Utilities|FlowControl|Delay 0.2)
      (Class|BPIChessInterface|CheckAllPieces(Message) _as_chess_game_state))))

(event Custom|KingInCheck?
  (bind _team (Variables|Default|GetTeam))
  (bind _team_2 (Variables|Default|GetTeam))
  (bind _as_chess_game_state (Variables|Default|GetAs%20Chess%20Game%20State))
  (bind _as_chess_game_state_2 (Variables|Default|GetAs%20Chess%20Game%20State))
  ;[1 1 1] King in-check Regular Testing
  (Utilities|Array|Clear (Variables|Default|GetValidMoves))
  (bind (_validmoves _checktiles _incheck_ _kingtile) (CallFunction|CheckPieceMoves))
  (Variables|Default|SetValidMoves _validmoves)
  (if _incheck_
    (switch int _team
      (:1
        (Default|KingCheckRelay _as_chess_game_state_2 (+ _team 1) true _checktiles _kingtile))
      (:2
        (Default|KingCheckRelay _as_chess_game_state_2 (- _team 1) true _checktiles _kingtile)))
    (else
      (Utilities|Array|Clear (Variables|Default|GetInCheckTiles))
      (switch int _team_2
        (:1
          (Default|KingCheckRelay _as_chess_game_state (+ _team_2 1) false _checktiles _kingtile))
        (:2
          (Default|KingCheckRelay _as_chess_game_state (- _team_2 1) false _checktiles _kingtile))))))

(event EventBeginPlay
  (Utilities|FlowControl|Sequence
    (:then_0
      (bind _aschess_game_mode (Utilities|Casting|CastToBP_ChessGameMode (Game|GetGameMode)))
      (Variables|Default|SetAs%20Chess%20Game%20Mode _aschess_game_mode))
    (:then_1
      (Utilities|FlowControl|Delay 1.0)
      (bind _outactors (Actor|GetAllActorsOfClass "/Game/MPChessTemplate/Blueprints/BP_Tile.BP_Tile_C"))
      (Variables|Default|SetOut%20Actors _outactors))
    (:then_2
      (bind _aschess_game_state (Utilities|Casting|CastToBP_ChessGameState (Game|GetGameState)))
      (Variables|Default|SetAs%20Chess%20Game%20State _aschess_game_state))
    (:then_3
      (Networking|SwitchHasAuthority
        (:Authority
          (Utilities|FlowControl|Delay 2.8)
          (CallFunction|KinginCheck?))))))

(event Collision|EventActorBeginOverlap
  (params (OtherActor :type Actor%20Object%20Reference)))

(event EventTick
  (params (DeltaSeconds :type Float%20%28single-precision%29)))

(event EventMovePiece
  (params (Piece :type BP%20Chess%20Pieces%20Object%20Reference) (Tile :type BP%20Tile%20Object%20Reference) (Number :type Integer) (Location :type Vector :default "0, 0, 0"))
  (bind _as_chess_game_state (Variables|Default|GetAs%20Chess%20Game%20State))
  (if (not (Variables|/Game/MPChessTemplate/Blueprints/BP_Tile.BP_Tile_C|GetKing? Tile))
    (bind _array_element (Utilities|Array|ForEachLoopwithBreak (Variables|Default|GetOut%20Actors) :!label _label)
      (:LoopBody
        (if (== (Variables|Default|GetCurrentTile) (Variables|/Game/MPChessTemplate/Blueprints/BP_Tile.BP_Tile_C|GetTileNumber _array_element))
          (Variables|/Game/MPChessTemplate/Blueprints/BP_Tile.BP_Tile_C|SetPiece _array_element 0)
          (Variables|Default|SetLastTile _array_element)
          (goto _label Break)))
      (:Completed
        ;[1 1 1] Regular Piece Move Command
        (bind _valid (CallFunction|PieceMoveLogic Number (Variables|/Game/MPChessTemplate/Blueprints/BP_Tile.BP_Tile_C|GetOccupied Tile) (Variables|Default|GetFirstMove?) (and (Variables|/Game/MPChessTemplate/Blueprints/BP_Tile.BP_Tile_C|GetOccupied Tile) (!= (Variables|Default|GetTeam) (Variables|/Game/MPChessTemplate/Blueprints/BP_Tile.BP_Tile_C|GetTeam Tile))) (Variables|Default|GetKingChecked)))
        (if _valid
          (if (Variables|/Game/MPChessTemplate/Blueprints/BP_Tile.BP_Tile_C|GetOccupied Tile)
            (if (!= (Variables|/Game/MPChessTemplate/Blueprints/BP_Tile.BP_Tile_C|GetTeam Tile) (Variables|Default|GetTeam))
              (bind _piece (Variables|/Game/MPChessTemplate/Blueprints/BP_Tile.BP_Tile_C|GetPiece Tile)
                (:then
                  (Default|DestroyPiece _piece))
                (:else
                  _))
              (CallFunction|SvrPieceMove Number Location Tile :!label _label_2)
              (Utilities|FlowControl|Sequence
                (:then_0
                  (Variables|Default|SetFirstMove? false)
                  (Variables|/Game/MPChessTemplate/Blueprints/BP_Tile.BP_Tile_C|SetPiece Tile self)
                  (Variables|/Game/MPChessTemplate/Blueprints/BP_Tile.BP_Tile_C|SetTeam Tile (Variables|Default|GetTeam))
                  (Variables|/Game/MPChessTemplate/Blueprints/BP_Tile.BP_Tile_C|SetOccupied (Variables|Default|GetLastTile) false))
                (:then_1
                  (Utilities|FlowControl|Delay 0.2)
                  (CallFunction|KinginCheck?)
                  (Default|CheckAllPieces (Variables|Default|GetAs%20Chess%20Game%20State) self)
                  (switch int (Variables|Default|GetTeam)
                    (:1
                      (Default|ChangeTurn _as_chess_game_state 2))
                    (:2
                      (Default|ChangeTurn _as_chess_game_state 1))))))
            (else
              (goto _label_2))))))))

(event EventDestroyPiece
  (params (Piece :type BP%20Chess%20Pieces%20Object%20Reference))
  ;[1 1 1] Piece Elimanation
  (CallFunction|SvrDestroyPiece self))

(event EventSelectPiece
  ;[1 1 1] Piece Selection
  (Rendering|SetVisibility (Variables|Default|GetDecal) true false))

(event EventDeselectPiece
  ;[1 1 1] Piece Selection
  (Rendering|SetVisibility (Variables|Default|GetDecal) false false))

(fn ConstructionScript)

(fn PieceMoveLogic
  (params (Tile :type Integer) (Occupied? :type Boolean) (FirstMove? :type Boolean) (EnemyOccupied? :type Boolean) (KingInCheck? :type Boolean))
  (return true false))

(fn EatEnemyPiece)

(fn CheckAvailable
  (params (Tiles :type Array%20of%20BP%20Tile%20Object%20References))
  (return 0))

(fn CheckPieceMoves
  (return 0 0 false 0 0))