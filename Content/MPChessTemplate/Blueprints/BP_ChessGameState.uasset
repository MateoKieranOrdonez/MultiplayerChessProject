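; Game state for multiplayer chess that builds the board, runs timed turns and decides match outcomes.
; Staggered delays at BeginPlay sequence server-side tile and data-table piece spawning, checkerboard materials and caching of pieces, player states and widgets.
; CheckAllPieces gathers each piece's check paths on the server, relaying them to pieces and player states and testing for checkmate or stalemate.
; It also spawns promoted pieces and randomly placed camera pawns.
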(event Custom|StartPoint
  (params (PlayerController :type BP%20Chess%20Player%20Controller%20Object%20Reference))
  (bind _startpoints (Variables|Default|GetStartPoints))
  (bind _outitem (Utilities|Array|Random _startpoints))
  ;[1 1 1] Camera
  (bind _returnvalue (Game|SpawnActorfromClass "/Game/MPChessTemplate/Blueprints/BP_CameraPawn.BP_CameraPawn_C" _outitem "Undefined" "MultiplyWithRoot" (Variables|/Script/Engine.Controller|GetPlayerState PlayerController) 0))
  (Utilities|Array|RemoveItem _startpoints _outitem)
  (Pawn|Possess PlayerController _returnvalue))

(event Custom|Checkmates_Stalemates
  (params (Checkmate? :type Boolean) (Team :type Integer))
  ;[1 1 1] Checkmates/Stalemates
  (Variables|Default|SetTotalMovesAvailableP1 0)
  (Variables|Default|SetTotalMovesAvailableP2 0)
  (Networking|SwitchHasAuthority
    (:Authority
      ;;[1 1 1] Check Total Valid Moves for all pieces
      (for _array_element (Variables|Default|GetChessPieces)
        (Utilities|IsValid _array_element
          (:Is%20Valid
            (switch int (Variables|/Game/MPChessTemplate/Blueprints/BP_ChessPieces.BP_ChessPieces_C|GetTeam _array_element)
              (:1
                (if (== (Utilities|GetClass _array_element) "/Game/MPChessTemplate/Blueprints/BP_King.BP_King_C")
                  (Variables|Default|SetKingLegalMovesP1 (Utilities|Array|IsEmpty (Variables|/Game/MPChessTemplate/Blueprints/BP_ChessPieces.BP_ChessPieces_C|GetValidMoves _array_element)))
                  (else
                    (Variables|Default|SetTotalMovesAvailableP1 (+ (Utilities|Array|Length (Variables|/Game/MPChessTemplate/Blueprints/BP_ChessPieces.BP_ChessPieces_C|GetValidMoves _array_element)) (Variables|Default|GetTotalMovesAvailableP1))))))
              (:2
                (if (== (Utilities|GetClass _array_element) "/Game/MPChessTemplate/Blueprints/BP_King.BP_King_C")
                  (Variables|Default|SetKingLegalMovesP2 (Utilities|Array|IsEmpty (Variables|/Game/MPChessTemplate/Blueprints/BP_ChessPieces.BP_ChessPieces_C|GetValidMoves _array_element)))
                  (else
                    (Variables|Default|SetTotalMovesAvailableP2 (+ (Utilities|Array|Length (Variables|/Game/MPChessTemplate/Blueprints/BP_ChessPieces.BP_ChessPieces_C|GetValidMoves _array_element)) (Variables|Default|GetTotalMovesAvailableP2))))))))))
      (if (Variables|Default|GetMatchStart)
        (switch int Team
          (:1
            (if (== (Variables|Default|GetTotalMovesAvailableP1) 0)
              (if (== (Variables|Default|GetKingLegalMovesP1) true)
                (if Checkmate?
                  (bind _array_element_2 (Utilities|Array|ForEachLoopwithBreak (Variables|Default|GetPlayerStates))
                    (:LoopBody
                      (Default|Mate _array_element_2 1)
                      (Default|MatchConclusion _array_element_2 2)))
                  (else
                    (bind _array_element_3 (Utilities|Array|ForEachLoopwithBreak (Variables|Default|GetPlayerStates) :!label _label)
                      (:LoopBody
                        (Default|Mate _array_element_3 2)
                        (Default|MatchConclusion _array_element_3))))))))
          (:2
            (if (== (Variables|Default|GetTotalMovesAvailableP2) 0)
              (if (== (Variables|Default|GetKingLegalMovesP2) true)
                (if Checkmate?
                  (bind _array_element_4 (Utilities|Array|ForEachLoopwithBreak (Variables|Default|GetPlayerStates))
                    (:LoopBody
                      (Default|Mate _array_element_4 1)
                      (Default|MatchConclusion _array_element_4 1)))
                  (else
                    (goto _label)))))))))))

(event Custom|SpawnPieces
  ;[1 1 1] Spawn Pieces
  (for _array_element (Variables|Default|GetOut%20Actors)
    (bind _outrownames (DataTable|GetDataTableRowNames "/Game/MPChessTemplate/Blueprints/DT_ChessPiecesDataTable.DT_ChessPiecesDataTable"))
    (for _array_element_2 _outrownames
      (bind _returnvalue (Utilities|GetDataTableRow "/Game/MPChessTemplate/Blueprints/DT_ChessPiecesDataTable.DT_ChessPiecesDataTable" _array_element_2)
        (:then
          (bind _array_element_3 (Utilities|Array|ForEachLoopwithBreak (.slots _returnvalue))
            (:LoopBody
              (if (== _array_element_3 (Variables|/Game/MPChessTemplate/Blueprints/BP_Tile.BP_Tile_C|GetTileNumber _array_element))
                (if (> (Variables|/Game/MPChessTemplate/Blueprints/BP_Tile.BP_Tile_C|GetTileNumber _array_element) 30)
                  (bind _returnvalue_2 (Game|SpawnActorfromClass (.piece _returnvalue) (Math|Transform|MakeTransform (Math|Vector|MakeVector (.X (Math|Vector|BreakVector (Transformation|GetActorLocation _array_element))) (.Y (Math|Vector|BreakVector (Transformation|GetActorLocation _array_element))) (+ (.Z (Math|Vector|BreakVector (Transformation|GetActorLocation _array_element))) 0.0)) "0.000000,180.000000,0.000000" "1.000000,1.000000,1.000000") "Undefined" "MultiplyWithRoot" 0 2 0 (Variables|/Game/MPChessTemplate/Blueprints/BP_Tile.BP_Tile_C|GetTileNumber _array_element) 0))
                  (Variables|/Game/MPChessTemplate/Blueprints/BP_Tile.BP_Tile_C|SetTeam _array_element 2)
                  (Variables|/Game/MPChessTemplate/Blueprints/BP_Tile.BP_Tile_C|SetPiece _array_element _returnvalue_2)
                  (if (== (Utilities|GetClass _returnvalue_2) "/Game/MPChessTemplate/Blueprints/BP_King.BP_King_C")
                    (Variables|/Game/MPChessTemplate/Blueprints/BP_Tile.BP_Tile_C|SetKing? _array_element true))
                  (else
                    (bind _returnvalue_3 (Game|SpawnActorfromClass (.piece _returnvalue) (Math|Transform|MakeTransform (Math|Vector|MakeVector (.X (Math|Vector|BreakVector (Transformation|GetActorLocation _array_element))) (.Y (Math|Vector|BreakVector (Transformation|GetActorLocation _array_element))) (+ (.Z (Math|Vector|BreakVector (Transformation|GetActorLocation _array_element))) 0.0)) "0, 0, 0" "1.000000,1.000000,1.000000") "Undefined" "MultiplyWithRoot" 0 1 0 (Variables|/Game/MPChessTemplate/Blueprints/BP_Tile.BP_Tile_C|GetTileNumber _array_element) 0))
                    (Variables|/Game/MPChessTemplate/Blueprints/BP_Tile.BP_Tile_C|SetTeam _array_element 1)
                    (Variables|/Game/MPChessTemplate/Blueprints/BP_Tile.BP_Tile_C|SetPiece _array_element _returnvalue_3)
                    (if (== (Utilities|GetClass _returnvalue_3) "/Game/MPChessTemplate/Blueprints/BP_King.BP_King_C")
                      (Variables|/Game/MPChessTemplate/Blueprints/BP_Tile.BP_Tile_C|SetKing? _array_element true))))
                (Variables|/Game/MPChessTemplate/Blueprints/BP_Tile.BP_Tile_C|SetOccupied _array_element true)))))))))

(event Custom|tiles
  ;[1 1 1] Set Tiles Material
  (bind _outactors (Actor|GetAllActorsOfClass "/Game/MPChessTemplate/Blueprints/BP_Tile.BP_Tile_C"))
  (for _array_element _outactors
    (Rendering|Material|SetMaterial (Variables|/Game/MPChessTemplate/Blueprints/BP_Tile.BP_Tile_C|GetTile _array_element) 0 (select (Class|KismetMathLibrary|XORBoolean (Math|Conversions|ToBoolean(Integer) (Math|Integer|%(Integer) (Variables|/Game/MPChessTemplate/Blueprints/BP_Tile.BP_Tile_C|GetTileNumber _array_element) 2)) (Math|Conversions|ToBoolean(Integer) (Math|Integer|%(Integer) (/ (Variables|/Game/MPChessTemplate/Blueprints/BP_Tile.BP_Tile_C|GetTileNumber _array_element) 8) 2))) "/Engine/EditorMaterials/GridMaterial.GridMaterial" "/Engine/BufferVisualization/BaseColor.BaseColor"))))

(event Custom|CheckNotifyPlayers
  (params (A :type Integer))
  ;[1 1 1] King in-Check
  ;;[1 1 1] Notify Playerstates of in-check states
  (bind _array_element (Utilities|Array|ForEachLoopwithBreak (Variables|Default|GetPlayerStates) :!label _label)
    (:LoopBody
      (if (== A (Variables|/Game/MPChessTemplate/Blueprints/BP_ChessPlayerState.BP_ChessPlayerState_C|GetTeam _array_element))
        (Utilities|FlowControl|Sequence
          (:then_0
            (goto _label Break))
          (:then_1
            (bind _array_element_2 (Utilities|Array|ForEachLoopwithBreak (Variables|Default|GetChessPieces) :!label _label_2)
              (:LoopBody
                (if (== A (Variables|/Game/MPChessTemplate/Blueprints/BP_ChessPieces.BP_ChessPieces_C|GetTeam _array_element_2))
                  (Variables|/Game/MPChessTemplate/Blueprints/BP_ChessPlayerState.BP_ChessPlayerState_C|SetInCheck _array_element (Variables|/Game/MPChessTemplate/Blueprints/BP_ChessPieces.BP_ChessPieces_C|GetKingChecked _array_element_2))
                  (goto _label_2 Break))))))))))

(event Custom|SpawnTiles
  ;[1 1 1] Spawn Tiles
  (for _index (range 0 63)
    (Game|SpawnActorfromClass "/Game/MPChessTemplate/Blueprints/BP_Tile.BP_Tile_C" (Math|Conversions|ToTransform(Vector) (Math|Vector|MakeVector (Math|Conversions|ToFloat(Integer) (* (/ _index 8) 1000)) (Math|Conversions|ToFloat(Integer) (* (Math|Integer|%(Integer) _index 8) 1000)) 0.0)) "Undefined" "MultiplyWithRoot" 0 _index 0 false 0 0 0)))

(event Custom|MatchBegin
  ;[0.15 0.15 0.15 0.5] Player 1 Turn
  (Utilities|FlowControl|Delay 5.0)
  (for _array_element (Variables|Default|GetFound%20Widgets)
    (Variables|/Script/UMG.TextBlock|SetText (Variables|/Game/MPChessTemplate/UI/WBP_UI.WBP_UI_C|GetYourTurn _array_element) "Match begins in 3 seconds"))
  (Utilities|FlowControl|Delay 3.0)
  (bind _array_element_2 (Utilities|Array|ForEachLoopwithBreak (Variables|Default|GetPlayerStates) :!label _label)
    (:LoopBody
      (if (== (Variables|/Game/MPChessTemplate/Blueprints/BP_ChessPlayerState.BP_ChessPlayerState_C|GetTeam _array_element_2) 1)
        (Variables|/Game/MPChessTemplate/Blueprints/BP_ChessPlayerState.BP_ChessPlayerState_C|SetMyTurn? _array_element_2 true)
        (goto _label Break)
        (else
          (Variables|/Game/MPChessTemplate/Blueprints/BP_ChessPlayerState.BP_ChessPlayerState_C|SetMyTurn? _array_element_2 false))))))

(event Custom|Changetrn
  (params (B :type Integer))
  ;[0.15 0.15 0.15 0.5] Change Turn
  (Variables|Default|SetTurnTimer (Variables|Default|GetTurnTIme))
  (bind _array_element (Utilities|Array|ForEachLoopwithBreak (Variables|Default|GetPlayerStates))
    (:LoopBody
      (if (== (Variables|/Game/MPChessTemplate/Blueprints/BP_ChessPlayerState.BP_ChessPlayerState_C|GetTeam _array_element) B)
        (Variables|/Game/MPChessTemplate/Blueprints/BP_ChessPlayerState.BP_ChessPlayerState_C|SetMyTurn? _array_element true)
        (else
          (Variables|Default|SetTeamTimer (Variables|/Game/MPChessTemplate/Blueprints/BP_ChessPlayerState.BP_ChessPlayerState_C|GetTeam _array_element))
          (Variables|/Game/MPChessTemplate/Blueprints/BP_ChessPlayerState.BP_ChessPlayerState_C|SetMyTurn? _array_element false))))
    (:Completed
      (Utilities|FlowControl|Delay 1.0 :!label _label)
      (bind _result (Math|Integer|DecrementInt (Variables|Default|GetTurnTimer))
        (:%20%20
          (bind _output_get (Variables|Default|SetTurnTimer _result))
          (for _array_element_2 (Variables|Default|GetFound%20Widgets)
            (Variables|/Script/UMG.TextBlock|SetText (Variables|/Game/MPChessTemplate/UI/WBP_UI.WBP_UI_C|GetTimer _array_element_2) (Utilities|Text|ToText(Integer) _output_get)))
          (if (<= _output_get 0)
            (CallFunction|ChangeTurn (Variables|Default|GetTeamTimer))
            (else
              (goto _label))))))))

(event EventBeginPlay
  (Utilities|FlowControl|Sequence
    (:then_0
      ;[1 1 1] Board & Pieces Setup
      (Networking|SwitchHasAuthority
        (:Authority
          (CallFunction|SpawnTiles))))
    (:then_1
      (Utilities|FlowControl|Delay 1.0)
      (bind _outactors (Actor|GetAllActorsOfClass "/Game/MPChessTemplate/Blueprints/BP_Tile.BP_Tile_C"))
      (Variables|Default|SetOut%20Actors _outactors)
      (Networking|SwitchHasAuthority
        (:Authority
          (CallFunction|SpawnPieces))))
    (:then_2
      (Utilities|FlowControl|Delay 2.0)
      (CallFunction|Tiles))
    (:then_3
      (Utilities|FlowControl|Delay 2.5)
      (bind _outactors_2 (Actor|GetAllActorsOfClass "/Game/MPChessTemplate/Blueprints/BP_ChessPieces.BP_ChessPieces_C"))
      (Variables|Default|SetChessPieces _outactors_2)
      (for _array_element _outactors_2
        (if (== (Variables|/Game/MPChessTemplate/Blueprints/BP_ChessPieces.BP_ChessPieces_C|GetTeam _array_element) 2)
          (Rendering|Material|SetMaterial (Variables|/Game/MPChessTemplate/Blueprints/BP_ChessPieces.BP_ChessPieces_C|GetStaticMesh _array_element) 0 "/Game/MPChessTemplate/Materials/M_Piece1.M_Piece1"))))
    (:then_4
      (Utilities|FlowControl|Delay 5.0)
      (bind _outactors_3 (Actor|GetAllActorsOfClass "/Game/MPChessTemplate/Blueprints/BP_ChessPlayerState.BP_ChessPlayerState_C"))
      (Variables|Default|SetPlayerStates _outactors_3))
    (:then_5
      ;[1 1 1] Match Begin
      (Utilities|FlowControl|Delay 5.0)
      (Variables|Default|SetMatchStart true)
      (bind _foundwidgets (Widget|GetAllWidgetsOfClass "/Game/MPChessTemplate/UI/WBP_UI.WBP_UI_C" false))
      (Variables|Default|SetFound%20Widgets _foundwidgets))
    (:then_6
      (Variables|Default|SetTurnTimer (Variables|Default|GetTurnTIme)))))

(event EventKingCheckRelay
  (params (Team :type Integer) (Check :type Boolean) (CheckPath :type Array%20of%20Integers) (KingTile :type BP%20Tile%20Object%20Reference))
  (bind _chesspieces (Variables|Default|GetChessPieces))
  ;[1 1 1] King in-Check
  ;;[1 1 1] Set In-Check State for Pieces
  (if Check
    (for _array_element _chesspieces
      (Utilities|IsValid _array_element
        (:Is%20Valid
          (if (== (Variables|/Game/MPChessTemplate/Blueprints/BP_ChessPieces.BP_ChessPieces_C|GetTeam _array_element) Team)
            (Variables|/Game/MPChessTemplate/Blueprints/BP_ChessPieces.BP_ChessPieces_C|SetInCheckTiles _array_element CheckPath)
            (Variables|/Game/MPChessTemplate/Blueprints/BP_ChessPieces.BP_ChessPieces_C|SetKingChecked _array_element true)))))
    (CallFunction|CheckmatesStalemates true Team)
    (CallFunction|CheckNotifyPlayers Team)
    (else
      (for _array_element_2 _chesspieces
        (Utilities|IsValid _array_element_2
          (:Is%20Valid
            (if (== (Variables|/Game/MPChessTemplate/Blueprints/BP_ChessPieces.BP_ChessPieces_C|GetTeam _array_element_2) Team)
              (Utilities|Array|Clear (Variables|/Game/MPChessTemplate/Blueprints/BP_ChessPieces.BP_ChessPieces_C|GetInCheckTiles _array_element_2))
              (Variables|/Game/MPChessTemplate/Blueprints/BP_ChessPieces.BP_ChessPieces_C|SetKingChecked _array_element_2 false)))))
      (CallFunction|CheckmatesStalemates false Team)
      (CallFunction|CheckNotifyPlayers Team))))

(event EventCheckAllPieces
  (params (Exception :type BP%20Chess%20Pieces%20Object%20Reference))
  ;[1 1 1] Checks Pieces Periodically
  (Utilities|Array|Clear (Variables|Default|GetP1Check))
  (Utilities|Array|Clear (Variables|Default|GetP2Check))
  (Utilities|Array|Clear (Variables|Default|GetP1CheckPath))
  (Utilities|Array|Clear (Variables|Default|GetP2CheckPath))
  (Networking|SwitchHasAuthority
    (:Authority
      (for _array_element (Variables|Default|GetChessPieces)
        (Utilities|IsValid _array_element
          (:Is%20Valid
            (Utilities|Array|Clear (Variables|/Game/MPChessTemplate/Blueprints/BP_ChessPieces.BP_ChessPieces_C|GetInCheckTiles _array_element))
            (bind (_validmoves _checktiles _incheck_) (Default|CheckPieceMoves _array_element))
            (if (== (Utilities|GetClass _array_element) "/Game/MPChessTemplate/Blueprints/BP_King.BP_King_C")
              (switch int (Variables|/Game/MPChessTemplate/Blueprints/BP_ChessPieces.BP_ChessPieces_C|GetTeam _array_element)
                (:1
                  (Utilities|Array|AddUnique (Variables|Default|GetP2Check) _incheck_)
                  (Utilities|Array|AppendArray (Variables|Default|GetP2CheckPath) _checktiles))
                (:2
                  (Utilities|Array|AddUnique (Variables|Default|GetP1Check) _incheck_)
                  (Utilities|Array|AppendArray (Variables|Default|GetP1CheckPath) _checktiles)))
              (else
                (switch int (Variables|/Game/MPChessTemplate/Blueprints/BP_ChessPieces.BP_ChessPieces_C|GetTeam _array_element)
                  (:1
                    (Utilities|Array|AddUnique (Variables|Default|GetP1Check) _incheck_)
                    (Utilities|Array|AppendArray (Variables|Default|GetP1CheckPath) _checktiles))
                  (:2
                    (Utilities|Array|AddUnique (Variables|Default|GetP2Check) _incheck_)
                    (Utilities|Array|AppendArray (Variables|Default|GetP2CheckPath) _checktiles))))))
          (:Is%20Not%20Valid
            (Development|PrintString "Hello"))))
      (if (Utilities|Array|ContainsItem (Variables|Default|GetP1Check) true)
        (CallFunction|KingCheckRelay 2 true (Variables|Default|GetP1CheckPath))
        (else
          (CallFunction|KingCheckRelay 2 false (Variables|Default|GetP1CheckPath))
          (if (Utilities|Array|ContainsItem (Variables|Default|GetP2Check) true)
            (CallFunction|KingCheckRelay 1 true (Variables|Default|GetP2CheckPath))
            (else
              (CallFunction|KingCheckRelay 1 false (Variables|Default|GetP2CheckPath)))))))))

(event EventDestroyPiece
  (params (Piece :type BP%20Chess%20Pieces%20Object%20Reference))
  (bind _chesspieces (Variables|Default|GetChessPieces))
  ;[1 1 1] Piece Elimination
  (bind _array_element (Utilities|Array|ForEachLoopwithBreak _chesspieces :!label _label)
    (:LoopBody
      (if (== _array_element Piece)
        (Utilities|Array|RemoveItem _chesspieces _array_element)
        (goto _label Break)))
    (:Completed
      (CallFunction|CheckAllPieces))))

(event EventChangeTurn
  (params (Team :type Integer))
  ;[0.15 0.15 0.15 0.5] Change Turn
  (CallFunction|Changetrn Team))

(event EventPawnPromotion
  (params (Class :type BP%20Chess%20Pieces%20Class%20Reference) (Team :type Integer) (Tile :type Integer))
  ;[1 1 1] Pawn Promotopn
  (for _array_element (Variables|Default|GetOut%20Actors)
    (if (== (Variables|/Game/MPChessTemplate/Blueprints/BP_Tile.BP_Tile_C|GetTileNumber _array_element) Tile)
      (switch int Team
        (:1
          (Game|SpawnActorfromClass Class (Math|Transform|MakeTransform (Math|Vector|MakeVector (.X (Math|Vector|BreakVector (Transformation|GetActorLocation _array_element))) (.Y (Math|Vector|BreakVector (Transformation|GetActorLocation _array_element))) (+ (.Z (Math|Vector|BreakVector (Transformation|GetActorLocation _array_element))) 1e+02)) "0.000000,180.000000,0.000000" "1.000000,1.000000,1.000000") "Undefined" "MultiplyWithRoot" 0 Team 0 Tile 0))
        (:2
          (Game|SpawnActorfromClass Class (Math|Transform|MakeTransform (Math|Vector|MakeVector (.X (Math|Vector|BreakVector (Transformation|GetActorLocation _array_element))) (.Y (Math|Vector|BreakVector (Transformation|GetActorLocation _array_element))) (+ (.Z (Math|Vector|BreakVector (Transformation|GetActorLocation _array_element))) 1e+02)) "0, 0, 0" "1.000000,1.000000,1.000000") "Undefined" "MultiplyWithRoot" 0 Team 0 Tile 0))))))

(event EventPawnProZone
  (params (Tile :type Integer) (Team :type Integer))
  ;[1 1 1] Pawn Promotopn
  (bind _array_element (Utilities|Array|ForEachLoopwithBreak (Variables|Default|GetPlayerStates) :!label _label)
    (:LoopBody
      (if (== (Variables|/Game/MPChessTemplate/Blueprints/BP_ChessPlayerState.BP_ChessPlayerState_C|GetTeam _array_element) Team)
        (Default|PawnProZone _array_element Tile Team)
        (goto _label Break)))))

(fn ConstructionScript)

(fn CheckAvailable
  (params (Tiles :type Array%20of%20BP%20Tile%20Object%20References))
  (return 0))

(fn CheckPieceMoves
  (return 0 0 false 0 0))