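; Bishop piece for a chess game, handling its diagonal movement rules on a 64-tile board.
; Each function walks the Steps offsets from CurrentTile, comparing row and column distance to the step count to prevent edge wrapping.
; PieceMoveLogic validates a target tile, restricted to InCheckTiles during check, and CheckAvailable lists reachable tiles.
; CheckPieceMoves gathers valid moves and reports check on the enemy king with the attack path.
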(event EventBeginPlay
  (|CallParentFunction) ; This node is disabled and will not be called.\nDrag off pins to build functionality.
)

(event Collision|EventActorBeginOverlap
  (params (OtherActor :type Actor%20Object%20Reference))
  (|CallParentFunction OtherActor) ; This node is disabled and will not be called.\nDrag off pins to build functionality.
)

(event EventTick
  (params (DeltaSeconds :type Float%20%28single-precision%29))
  (|CallParentFunction DeltaSeconds) ; This node is disabled and will not be called.\nDrag off pins to build functionality.
)

(fn ConstructionScript
  (|CallParentFunction))

(fn PieceMoveLogic
  (params (Tile :type Integer) (Occupied? :type Boolean) (FirstMove? :type Boolean) (EnemyOccupied? :type Boolean) (KingInCheck? :type Boolean))
  (bind _newlocalvar (LocalVariables|GetNewLocalVar))
  (bind _newlocalvar_2 (LocalVariables|GetNewLocalVar))
  (bind _currenttile (Variables|Default|GetCurrentTile))
  (bind _returnvalue (Utilities|Array|ContainsItem _newlocalvar Tile))
  ;[1 1 1] Per StepDirecton
  (for _array_element (LocalVariables|GetSteps)
    (bind _output_get (LocalVariables|SetStepCount 1))
    (LocalVariables|SetDynamic (+ (Variables|Default|GetCurrentTile) (* _array_element _output_get)))
    ;[1 1 1] If within board range
    (for _index (range 0 63)
      (LocalVariables|SetDynamic (+ (Variables|Default|GetCurrentTile) (* _array_element (LocalVariables|GetStepCount))))
      (if (not (or (!= (Math|Integer|Absolute(Integer) (- (Math|Integer|%(Integer) (LocalVariables|GetDynamic) 8) (Math|Integer|%(Integer) _currenttile 8))) (LocalVariables|GetStepCount)) (!= (Math|Integer|Absolute(Integer) (- (/ (LocalVariables|GetDynamic) 8) (/ _currenttile 8))) (LocalVariables|GetStepCount))))
        ;[1 1 1] Check if the tile is occupied
        (bind _array_element_2 (Utilities|Array|ForEachLoopwithBreak (Variables|Default|GetOut%20Actors) :!label _label)
          (:LoopBody
            (if (== (Variables|/Game/MPChessTemplate/Blueprints/BP_Tile.BP_Tile_C|GetTileNumber _array_element_2) (LocalVariables|GetDynamic))
              (if (Variables|/Game/MPChessTemplate/Blueprints/BP_Tile.BP_Tile_C|GetOccupied _array_element_2)
                (if (== (Variables|/Game/MPChessTemplate/Blueprints/BP_Tile.BP_Tile_C|GetTeam _array_element_2) (Variables|Default|GetTeam))
                  _
                  (else
                    _))
                (Utilities|Array|AddUnique _newlocalvar_2 (LocalVariables|GetDynamic))
                (goto _label Break)
                (else
                  (Utilities|Array|AddUnique _newlocalvar_2 (LocalVariables|GetDynamic))
                  (bind _result (Math|Integer|IncrementInt (LocalVariables|GetStepCount))
                    (:%20%20
                      (LocalVariables|SetStepCount _result)))))))))))
  (if KingInCheck?
    (if (and (Utilities|Array|ContainsItem (Variables|Default|GetInCheckTiles) Tile) _returnvalue)
      _
      (else
        (return false false)))
    (elif _returnvalue
      _
      (else
        (return false false))))
  (return true false))

(fn CheckAvailable
  (params (Tiles :type Array%20of%20BP%20Tile%20Object%20References))
  (bind _localopentiles (LocalVariables|GetLocalOpenTIles))
  (bind _currenttile (Variables|Default|GetCurrentTile))
  ;[1 1 1] Per StepDirecton
  (for _array_element (LocalVariables|GetSteps)
    (bind _output_get (LocalVariables|SetStepCount 1))
    (LocalVariables|SetDynamic (+ (Variables|Default|GetCurrentTile) (* _array_element _output_get)))
    ;[1 1 1] If within board range
    (for _index (range 0 63)
      (LocalVariables|SetDynamic (+ (Variables|Default|GetCurrentTile) (* _array_element (LocalVariables|GetStepCount))))
      (if (not (or (!= (Math|Integer|Absolute(Integer) (- (Math|Integer|%(Integer) (LocalVariables|GetDynamic) 8) (Math|Integer|%(Integer) _currenttile 8))) (LocalVariables|GetStepCount)) (!= (Math|Integer|Absolute(Integer) (- (/ (LocalVariables|GetDynamic) 8) (/ _currenttile 8))) (LocalVariables|GetStepCount))))
        ;[1 1 1] Check if the tile is occupied
        (bind _array_element_2 (Utilities|Array|ForEachLoopwithBreak Tiles :!label _label)
          (:LoopBody
            (if (== (Variables|/Game/MPChessTemplate/Blueprints/BP_Tile.BP_Tile_C|GetTileNumber _array_element_2) (LocalVariables|GetDynamic))
              (if (Variables|/Game/MPChessTemplate/Blueprints/BP_Tile.BP_Tile_C|GetOccupied _array_element_2)
                (if (not (== (Variables|/Game/MPChessTemplate/Blueprints/BP_Tile.BP_Tile_C|GetTeam _array_element_2) (Variables|Default|GetTeam)))
                  (Utilities|Array|AddUnique _localopentiles (LocalVariables|GetDynamic))
                  (goto _label Break))
                (else
                  (Utilities|Array|AddUnique _localopentiles (LocalVariables|GetDynamic))
                  (bind _result (Math|Integer|IncrementInt (LocalVariables|GetStepCount))
                    (:%20%20
                      (LocalVariables|SetStepCount _result)))))))))))
  (return (LocalVariables|GetLocalOpenTIles)))

(fn CheckPieceMoves
  (bind _currenttile (Variables|Default|GetCurrentTile))
  (bind _inchecktiles (Variables|Default|GetInCheckTiles))
  (bind _validmoves (Variables|Default|GetValidMoves))
  (bind _validmoves_2 (Variables|Default|GetValidMoves))
  (Utilities|Array|Clear (LocalVariables|GetKinginCheck?))
  (LocalVariables|SetKingPosition 0)
  ;[1 1 1] Per StepDirecton
  (for _array_element (LocalVariables|GetSteps)
    (bind _output_get (LocalVariables|SetStepCount 1))
    (LocalVariables|SetDynamic (+ (Variables|Default|GetCurrentTile) (* _array_element _output_get)))
    (Utilities|Array|Clear (LocalVariables|GetTempPath))
    ;[1 1 1] If within board range
    (for _index (range 0 63)
      (LocalVariables|SetDynamic (+ (Variables|Default|GetCurrentTile) (* _array_element (LocalVariables|GetStepCount))))
      (if (or (!= (Math|Integer|Absolute(Integer) (- (Math|Integer|%(Integer) (LocalVariables|GetDynamic) 8) (Math|Integer|%(Integer) _currenttile 8))) (LocalVariables|GetStepCount)) (!= (Math|Integer|Absolute(Integer) (- (/ (LocalVariables|GetDynamic) 8) (/ _currenttile 8))) (LocalVariables|GetStepCount)))
        (Utilities|Array|Clear (LocalVariables|GetTempPath))
        (else
          ;[1 1 1] Check if the tile is occupied
          (bind _array_element_2 (Utilities|Array|ForEachLoopwithBreak (Variables|Default|GetOut%20Actors) :!label _label)
            (:LoopBody
              (if (== (Variables|/Game/MPChessTemplate/Blueprints/BP_Tile.BP_Tile_C|GetTileNumber _array_element_2) (LocalVariables|GetDynamic))
                (if (Variables|/Game/MPChessTemplate/Blueprints/BP_Tile.BP_Tile_C|GetOccupied _array_element_2)
                  (if (== (Variables|/Game/MPChessTemplate/Blueprints/BP_Tile.BP_Tile_C|GetTeam _array_element_2) (Variables|Default|GetTeam))
                    (goto _label Break)
                    (else
                      (Utilities|Array|AddUnique _validmoves (LocalVariables|GetDynamic))
                      ;[1 1 1] For King Check
                      (Utilities|Array|AddUnique (LocalVariables|GetKinginCheck?) (Variables|/Game/MPChessTemplate/Blueprints/BP_Tile.BP_Tile_C|GetKing? _array_element_2))
                      (if (Variables|/Game/MPChessTemplate/Blueprints/BP_Tile.BP_Tile_C|GetKing? _array_element_2)
                        (LocalVariables|SetKingPosition _array_element_2)
                        (Utilities|Array|AppendArray (Variables|Default|GetInCheckTiles) (LocalVariables|GetTempPath)))
                      (Utilities|Array|Clear (LocalVariables|GetTempPath))
                      (goto _label Break)))
                  (else
                    (Utilities|Array|AddUnique _validmoves (LocalVariables|GetDynamic))
                    (Utilities|Array|AddUnique (LocalVariables|GetTempPath) (LocalVariables|GetDynamic))
                    (bind _result (Math|Integer|IncrementInt (LocalVariables|GetStepCount))
                      (:%20%20
                        (LocalVariables|SetStepCount _result))))))))))))
  (if (Utilities|Array|ContainsItem (LocalVariables|GetKinginCheck?) true)
    (Utilities|Array|AddUnique _inchecktiles (Variables|Default|GetCurrentTile))
    (return _validmoves_2 _inchecktiles true (LocalVariables|GetKingPosition) 0)
    (else
      (return _validmoves_2 0 false 0 0))))