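; BP_Queen is the queen piece for a chess game, computing where it can move on an 8x8 tile board.
; Its functions walk each Steps offset as a ray, using modulo and division to prevent edge wrapping and tile occupancy to find captures and blockers.
; CheckPieceMoves also reports check, the king's tile and the attack path.
; PieceMoveLogic validates a target tile, limited to InCheckTiles when the king is in check.
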(event EventBeginPlay
  (|CallParentFunction) ; This node is disabled and will not be called.\nDrag off pins to build functionality.
)

(event Collision|EventActorBeginOverlap
  (params (OtherActor :type Actor%20Object%20Reference))
  (|CallParentFunction OtherActor) ; This node is disabled and will not be called.\nDrag off pins to build functionality.
)

(event EventTick
  (params (DeltaSeconds :type Float%20%28single-precision%29))
  (|CallParentFunction DeltaSeconds) ; This node is disabled and will not be called.\nDrag off pins to build functionality.
)

(fn ConstructionScript
  (|CallParentFunction))

(fn CheckAvailable
  (params (Tiles :type Array%20of%20BP%20Tile%20Object%20References))
  (bind _currenttile (Variables|Default|GetCurrentTile))
  (bind _localopentiles (LocalVariables|GetLocalOpenTIles))
  (bind _currenttile_2 (Variables|Default|GetCurrentTile))
  (bind _returnvalue (Math|Integer|%(Integer) _currenttile 8))
  (bind _returnvalue_2 (/ _currenttile 8))
  ;[1 1 1] Per StepDirecton
  (for _array_element (LocalVariables|GetSteps)
    (bind _output_get (LocalVariables|SetStepCount 1))
    (LocalVariables|SetDynamic (+ (Variables|Default|GetCurrentTile) (* _array_element _output_get)))
    (if (or (== (Math|Integer|Absolute(Integer) _array_element) 7) (== (Math|Integer|Absolute(Integer) _array_element) 9))
      ;[1 1 1] If within board range
      (for _index (range 0 63)
        (LocalVariables|SetDynamic (+ (Variables|Default|GetCurrentTile) (* _array_element (LocalVariables|GetStepCount))))
        ;[1 1 1] Get Next Tile Without warping (Diagonal)
        (if (not (or (!= (Math|Integer|Absolute(Integer) (- (Math|Integer|%(Integer) (LocalVariables|GetDynamic) 8) (Math|Integer|%(Integer) _currenttile_2 8))) (LocalVariables|GetStepCount)) (!= (Math|Integer|Absolute(Integer) (- (/ (LocalVariables|GetDynamic) 8) (/ _currenttile_2 8))) (LocalVariables|GetStepCount))))
          ;[1 1 1] Check if the tile is occupied
          (bind _array_element_2 (Utilities|Array|ForEachLoopwithBreak Tiles :!label _label)
            (:LoopBody
              (if (== (Variables|/Game/MPChessTemplate/Blueprints/BP_Tile.BP_Tile_C|GetTileNumber _array_element_2) (LocalVariables|GetDynamic))
                (if (Variables|/Game/MPChessTemplate/Blueprints/BP_Tile.BP_Tile_C|GetOccupied _array_element_2)
                  (if (not (== (Variables|/Game/MPChessTemplate/Blueprints/BP_Tile.BP_Tile_C|GetTeam _array_element_2) (Variables|Default|GetTeam)))
                    (Utilities|Array|AddUnique _localopentiles (LocalVariables|GetDynamic))
                    (goto _label Break))
                  (else
                    (Utilities|Array|AddUnique _localopentiles (LocalVariables|GetDynamic))
                    (bind _result (Math|Integer|IncrementInt (LocalVariables|GetStepCount))
                      (:%20%20
                        (LocalVariables|SetStepCount _result))))))))))
      (else
        ;[1 1 1] If within board range
        (for _index_2 (range 0 63)
          (LocalVariables|SetDynamic (+ (Variables|Default|GetCurrentTile) (* _array_element (LocalVariables|GetStepCount))))
          ;[1 1 1] Get the next tile without warping (Straight)
          (if (or (and (== (Math|Integer|%(Integer) (LocalVariables|GetDynamic) 8) _returnvalue) (!= _returnvalue_2 (/ (LocalVariables|GetDynamic) 8))) (and (== _returnvalue_2 (/ (LocalVariables|GetDynamic) 8)) (!= _returnvalue (Math|Integer|%(Integer) (LocalVariables|GetDynamic) 8))))
            (bind _array_element_3 (Utilities|Array|ForEachLoopwithBreak Tiles :!label _label_2)
              (:LoopBody
                (if (== (Variables|/Game/MPChessTemplate/Blueprints/BP_Tile.BP_Tile_C|GetTileNumber _array_element_3) (LocalVariables|GetDynamic))
                  (if (Variables|/Game/MPChessTemplate/Blueprints/BP_Tile.BP_Tile_C|GetOccupied _array_element_3)
                    (if (not (== (Variables|/Game/MPChessTemplate/Blueprints/BP_Tile.BP_Tile_C|GetTeam _array_element_3) (Variables|Default|GetTeam)))
                      (Utilities|Array|AddUnique _localopentiles (LocalVariables|GetDynamic))
                      (goto _label_2 Break))
                    (else
                      (Utilities|Array|AddUnique _localopentiles (LocalVariables|GetDynamic))
                      (bind _result_2 (Math|Integer|IncrementInt (LocalVariables|GetStepCount))
                        (:%20%20
                          (LocalVariables|SetStepCount _result_2)))))))))))))
  (return (LocalVariables|GetLocalOpenTIles)))

(fn PieceMoveLogic
  (params (Tile :type Integer) (Occupied? :type Boolean) (FirstMove? :type Boolean) (EnemyOccupied? :type Boolean) (KingInCheck? :type Boolean))
  (bind _currenttile (Variables|Default|GetCurrentTile))
  (bind _localopentiles (LocalVariables|GetLocalOpenTIles))
  (bind _currenttile_2 (Variables|Default|GetCurrentTile))
  (bind _localopentiles_2 (LocalVariables|GetLocalOpenTIles))
  (bind _returnvalue (Utilities|Array|ContainsItem _localopentiles_2 Tile))
  (bind _returnvalue_2 (Math|Integer|%(Integer) _currenttile 8))
  (bind _returnvalue_3 (/ _currenttile 8))
  ;[1 1 1] Per StepDirecton
  (for _array_element (LocalVariables|GetSteps)
    (bind _output_get (LocalVariables|SetStepCount 1))
    (LocalVariables|SetDynamic (+ (Variables|Default|GetCurrentTile) (* _array_element _output_get)))
    (if (or (== (Math|Integer|Absolute(Integer) _array_element) 7) (== (Math|Integer|Absolute(Integer) _array_element) 9))
      ;[1 1 1] If within board range
      (for _index (range 0 63)
        (LocalVariables|SetDynamic (+ (Variables|Default|GetCurrentTile) (* _array_element (LocalVariables|GetStepCount))))
        ;[1 1 1] Get Next Tile Without warping (Diagonal)
        (if (not (or (!= (Math|Integer|Absolute(Integer) (- (Math|Integer|%(Integer) (LocalVariables|GetDynamic) 8) (Math|Integer|%(Integer) _currenttile_2 8))) (LocalVariables|GetStepCount)) (!= (Math|Integer|Absolute(Integer) (- (/ (LocalVariables|GetDynamic) 8) (/ _currenttile_2 8))) (LocalVariables|GetStepCount))))
          ;[1 1 1] Check if the tile is occupied
          (bind _array_element_2 (Utilities|Array|ForEachLoopwithBreak (Variables|Default|GetOut%20Actors) :!label _label)
            (:LoopBody
              (if (== (Variables|/Game/MPChessTemplate/Blueprints/BP_Tile.BP_Tile_C|GetTileNumber _array_element_2) (LocalVariables|GetDynamic))
                (if (Variables|/Game/MPChessTemplate/Blueprints/BP_Tile.BP_Tile_C|GetOccupied _array_element_2)
                  (if (not (== (Variables|/Game/MPChessTemplate/Blueprints/BP_Tile.BP_Tile_C|GetTeam _array_element_2) (Variables|Default|GetTeam)))
                    (Utilities|Array|AddUnique _localopentiles (LocalVariables|GetDynamic))
                    (goto _label Break))
                  (else
                    (Utilities|Array|AddUnique _localopentiles (LocalVariables|GetDynamic))
                    (bind _result (Math|Integer|IncrementInt (LocalVariables|GetStepCount))
                      (:%20%20
                        (LocalVariables|SetStepCount _result))))))))))
      (else
        ;[1 1 1] If within board range
        (for _index_2 (range 0 63)
          (LocalVariables|SetDynamic (+ (Variables|Default|GetCurrentTile) (* _array_element (LocalVariables|GetStepCount))))
          ;[1 1 1] Get the next tile without warping (Straight)
          (if (or (and (== (Math|Integer|%(Integer) (LocalVariables|GetDynamic) 8) _returnvalue_2) (!= _returnvalue_3 (/ (LocalVariables|GetDynamic) 8))) (and (== _returnvalue_3 (/ (LocalVariables|GetDynamic) 8)) (!= _returnvalue_2 (Math|Integer|%(Integer) (LocalVariables|GetDynamic) 8))))
            (bind _array_element_3 (Utilities|Array|ForEachLoopwithBreak (Variables|Default|GetOut%20Actors) :!label _label_2)
              (:LoopBody
                (if (== (Variables|/Game/MPChessTemplate/Blueprints/BP_Tile.BP_Tile_C|GetTileNumber _array_element_3) (LocalVariables|GetDynamic))
                  (if (Variables|/Game/MPChessTemplate/Blueprints/BP_Tile.BP_Tile_C|GetOccupied _array_element_3)
                    (if (not (== (Variables|/Game/MPChessTemplate/Blueprints/BP_Tile.BP_Tile_C|GetTeam _array_element_3) (Variables|Default|GetTeam)))
                      (Utilities|Array|AddUnique _localopentiles (LocalVariables|GetDynamic))
                      (goto _label_2 Break))
                    (else
                      (Utilities|Array|AddUnique _localopentiles (LocalVariables|GetDynamic))
                      (bind _result_2 (Math|Integer|IncrementInt (LocalVariables|GetStepCount))
                        (:%20%20
                          (LocalVariables|SetStepCount _result_2)))))))))))))
  (if KingInCheck?
    (if (and (Utilities|Array|ContainsItem (Variables|Default|GetInCheckTiles) Tile) _returnvalue)
      _
      (else
        (return false false)))
    (elif _returnvalue
      _
      (else
        (return false false))))
  (return true false))

(fn CheckMoves
  (params (Tiles :type Array%20of%20BP%20Tile%20Object%20References))
  (bind _currenttile (Variables|Default|GetCurrentTile))
  (bind _currenttile_2 (Variables|Default|GetCurrentTile))
  (bind _validmoves (Variables|Default|GetValidMoves))
  (bind _returnvalue (Math|Integer|%(Integer) _currenttile 8))
  (bind _returnvalue_2 (/ _currenttile 8))
  (Utilities|Array|Clear (LocalVariables|GetKingInCheck))
  ;[1 1 1] Per StepDirecton
  (for _array_element (LocalVariables|GetSteps)
    (bind _output_get (LocalVariables|SetStepCount 1))
    (LocalVariables|SetDynamic (+ (Variables|Default|GetCurrentTile) (* _array_element _output_get)))
    (if (or (== (Math|Integer|Absolute(Integer) _array_element) 7) (== (Math|Integer|Absolute(Integer) _array_element) 9))
      ;[1 1 1] If within board range
      (for _index (range 0 63)
        (LocalVariables|SetDynamic (+ (Variables|Default|GetCurrentTile) (* _array_element (LocalVariables|GetStepCount))))
        ;[1 1 1] Get Next Tile Without warping (Diagonal)
        (if (not (or (!= (Math|Integer|Absolute(Integer) (- (Math|Integer|%(Integer) (LocalVariables|GetDynamic) 8) (Math|Integer|%(Integer) _currenttile_2 8))) (LocalVariables|GetStepCount)) (!= (Math|Integer|Absolute(Integer) (- (/ (LocalVariables|GetDynamic) 8) (/ _currenttile_2 8))) (LocalVariables|GetStepCount))))
          ;[1 1 1] Check if the tile is occupied
          (bind _array_element_2 (Utilities|Array|ForEachLoopwithBreak (Variables|Default|GetOut%20Actors) :!label _label)
            (:LoopBody
              (if (== (Variables|/Game/MPChessTemplate/Blueprints/BP_Tile.BP_Tile_C|GetTileNumber _array_element_2) (LocalVariables|GetDynamic))
                (if (Variables|/Game/MPChessTemplate/Blueprints/BP_Tile.BP_Tile_C|GetOccupied _array_element_2)
                  (if (not (== (Variables|/Game/MPChessTemplate/Blueprints/BP_Tile.BP_Tile_C|GetTeam _array_element_2) (Variables|Default|GetTeam)))
                    (Utilities|Array|AddUnique _validmoves (LocalVariables|GetDynamic))
                    (Development|PrintString (Utilities|String|ToString(Boolean) (Variables|/Game/MPChessTemplate/Blueprints/BP_Tile.BP_Tile_C|GetKing? _array_element_2)) true true "(R=0.000000,G=0.660000,B=1.000000,A=1.000000)" 1e+01)
                    (goto _label Break))
                  (else
                    (Utilities|Array|AddUnique _validmoves (LocalVariables|GetDynamic))
                    (bind _result (Math|Integer|IncrementInt (LocalVariables|GetStepCount))
                      (:%20%20
                        (LocalVariables|SetStepCount _result))))))))))
      (else
        ;[1 1 1] If within board range
        (for _index_2 (range 0 63)
          (LocalVariables|SetDynamic (+ (Variables|Default|GetCurrentTile) (* _array_element (LocalVariables|GetStepCount))))
          ;[1 1 1] Get the next tile without warping (Straight)
          (if (or (and (== (Math|Integer|%(Integer) (LocalVariables|GetDynamic) 8) _returnvalue) (!= _returnvalue_2 (/ (LocalVariables|GetDynamic) 8))) (and (== _returnvalue_2 (/ (LocalVariables|GetDynamic) 8)) (!= _returnvalue (Math|Integer|%(Integer) (LocalVariables|GetDynamic) 8))))
            (bind _array_element_3 (Utilities|Array|ForEachLoopwithBreak (Variables|Default|GetOut%20Actors) :!label _label_2)
              (:LoopBody
                (if (== (Variables|/Game/MPChessTemplate/Blueprints/BP_Tile.BP_Tile_C|GetTileNumber _array_element_3) (LocalVariables|GetDynamic))
                  (if (Variables|/Game/MPChessTemplate/Blueprints/BP_Tile.BP_Tile_C|GetOccupied _array_element_3)
                    (if (not (== (Variables|/Game/MPChessTemplate/Blueprints/BP_Tile.BP_Tile_C|GetTeam _array_element_3) (Variables|Default|GetTeam)))
                      (Utilities|Array|AddUnique _validmoves (LocalVariables|GetDynamic))
                      (Development|PrintString (Utilities|String|ToString(Boolean) (Variables|/Game/MPChessTemplate/Blueprints/BP_Tile.BP_Tile_C|GetKing? _array_element_3)) true true "(R=0.000000,G=0.660000,B=1.000000,A=1.000000)" 1e+01)
                      (goto _label_2 Break))
                    (else
                      (Utilities|Array|AddUnique _validmoves (LocalVariables|GetDynamic))
                      (bind _result_2 (Math|Integer|IncrementInt (LocalVariables|GetStepCount))
                        (:%20%20
                          (LocalVariables|SetStepCount _result_2)))))))))))))
  (return (Variables|Default|GetValidMoves) false 0))

(fn CheckPieceMoves
  (bind _currenttile (Variables|Default|GetCurrentTile))
  (bind _inchecktiles (Variables|Default|GetInCheckTiles))
  (bind _currenttile_2 (Variables|Default|GetCurrentTile))
  (bind _validmoves (Variables|Default|GetValidMoves))
  (bind _validmoves_2 (Variables|Default|GetValidMoves))
  (bind _returnvalue (Math|Integer|%(Integer) _currenttile 8))
  (bind _returnvalue_2 (/ _currenttile 8))
  (Utilities|Array|Clear (LocalVariables|GetKinginCheck?))
  ;[1 1 1] Per StepDirecton
  (for _array_element (LocalVariables|GetSteps)
    (bind _output_get (LocalVariables|SetStepCount 1))
    (LocalVariables|SetDynamic (+ (Variables|Default|GetCurrentTile) (* _array_element _output_get)))
    (if (or (== (Math|Integer|Absolute(Integer) _array_element) 7) (== (Math|Integer|Absolute(Integer) _array_element) 9))
      (Utilities|Array|Clear (LocalVariables|GetTempPath))
      ;[1 1 1] If within board range
      (for _index (range 0 63)
        (LocalVariables|SetDynamic (+ (Variables|Default|GetCurrentTile) (* _array_element (LocalVariables|GetStepCount))))
        ;[1 1 1] Get Next Tile Without warping (Diagonal)
        (if (or (!= (Math|Integer|Absolute(Integer) (- (Math|Integer|%(Integer) (LocalVariables|GetDynamic) 8) (Math|Integer|%(Integer) _currenttile_2 8))) (LocalVariables|GetStepCount)) (!= (Math|Integer|Absolute(Integer) (- (/ (LocalVariables|GetDynamic) 8) (/ _currenttile_2 8))) (LocalVariables|GetStepCount)))
          (Utilities|Array|Clear (LocalVariables|GetTempPath))
          (else
            ;[1 1 1] Check if the tile is occupied
            (bind _array_element_2 (Utilities|Array|ForEachLoopwithBreak (Variables|Default|GetOut%20Actors) :!label _label)
              (:LoopBody
                (if (== (Variables|/Game/MPChessTemplate/Blueprints/BP_Tile.BP_Tile_C|GetTileNumber _array_element_2) (LocalVariables|GetDynamic))
                  (if (Variables|/Game/MPChessTemplate/Blueprints/BP_Tile.BP_Tile_C|GetOccupied _array_element_2)
                    (if (== (Variables|/Game/MPChessTemplate/Blueprints/BP_Tile.BP_Tile_C|GetTeam _array_element_2) (Variables|Default|GetTeam))
                      (goto _label Break)
                      (else
                        (Utilities|Array|AddUnique _validmoves_2 (LocalVariables|GetDynamic))
                        ;;[1 1 1] For King Check
                        (Utilities|Array|AddUnique (LocalVariables|GetKinginCheck?) (Variables|/Game/MPChessTemplate/Blueprints/BP_Tile.BP_Tile_C|GetKing? _array_element_2))
                        (if (Variables|/Game/MPChessTemplate/Blueprints/BP_Tile.BP_Tile_C|GetKing? _array_element_2)
                          (LocalVariables|SetKingPosition _array_element_2)
                          (Utilities|Array|AppendArray (Variables|Default|GetInCheckTiles) (LocalVariables|GetTempPath)))
                        (Utilities|Array|Clear (LocalVariables|GetTempPath))
                        (goto _label Break)))
                    (else
                      (Utilities|Array|AddUnique _validmoves_2 (LocalVariables|GetDynamic))
                      (Utilities|Array|AddUnique (LocalVariables|GetTempPath) (LocalVariables|GetDynamic))
                      (bind _result (Math|Integer|IncrementInt (LocalVariables|GetStepCount))
                        (:%20%20
                          (LocalVariables|SetStepCount _result)))))))))))
      (else
        ;[1 1 1] If within board range
        (for _index_2 (range 0 63)
          (LocalVariables|SetDynamic (+ (Variables|Default|GetCurrentTile) (* _array_element (LocalVariables|GetStepCount))))
          ;[1 1 1] Get the next tile without warping (Straight)
          (if (or (and (== (Math|Integer|%(Integer) (LocalVariables|GetDynamic) 8) _returnvalue) (!= _returnvalue_2 (/ (LocalVariables|GetDynamic) 8))) (and (== _returnvalue_2 (/ (LocalVariables|GetDynamic) 8)) (!= _returnvalue (Math|Integer|%(Integer) (LocalVariables|GetDynamic) 8))))
            (bind _array_element_3 (Utilities|Array|ForEachLoopwithBreak (Variables|Default|GetOut%20Actors) :!label _label_2)
              (:LoopBody
                (if (== (Variables|/Game/MPChessTemplate/Blueprints/BP_Tile.BP_Tile_C|GetTileNumber _array_element_3) (LocalVariables|GetDynamic))
                  (if (Variables|/Game/MPChessTemplate/Blueprints/BP_Tile.BP_Tile_C|GetOccupied _array_element_3)
                    (if (== (Variables|/Game/MPChessTemplate/Blueprints/BP_Tile.BP_Tile_C|GetTeam _array_element_3) (Variables|Default|GetTeam))
                      (goto _label_2 Break)
                      (else
                        (Utilities|Array|AddUnique _validmoves_2 (LocalVariables|GetDynamic))
                        (Utilities|Array|AddUnique (LocalVariables|GetKinginCheck?) (Variables|/Game/MPChessTemplate/Blueprints/BP_Tile.BP_Tile_C|GetKing? _array_element_3))
                        (if (Variables|/Game/MPChessTemplate/Blueprints/BP_Tile.BP_Tile_C|GetKing? _array_element_3)
                          (LocalVariables|SetKingPosition _array_element_3)
                          (Utilities|Array|AppendArray (Variables|Default|GetInCheckTiles) (LocalVariables|GetTempPath)))
                        (Utilities|Array|Clear (LocalVariables|GetTempPath))
                        (goto _label_2 Break)))
                    (else
                      (Utilities|Array|AddUnique _validmoves_2 (LocalVariables|GetDynamic))
                      (Utilities|Array|AddUnique (LocalVariables|GetTempPath) (LocalVariables|GetDynamic))
                      (bind _result_2 (Math|Integer|IncrementInt (LocalVariables|GetStepCount))
                        (:%20%20
                          (LocalVariables|SetStepCount _result_2))))))))
            (else
              (Utilities|Array|Clear (LocalVariables|GetTempPath))))))))
  (if (Utilities|Array|ContainsItem (LocalVariables|GetKinginCheck?) true)
    (Utilities|Array|AddUnique _inchecktiles (Variables|Default|GetCurrentTile))
    (return _validmoves _inchecktiles true (LocalVariables|GetKingPosition) 0)
    (else
      (return _validmoves 0 false 0 0))))