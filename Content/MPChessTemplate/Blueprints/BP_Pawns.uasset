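; Pawn piece for a multiplayer chess game, handling movement, capture, check detection and promotion for both teams.
; MovePiece validates with PieceMoveLogic, captures, calls SvrPieceMove, then triggers game-state check scans and promotion.
; Rules use tile-number offsets per team, limited to InCheckTiles while in check; the two-tile first move ignores the intermediate tile.
; CheckAvailable lists open moves, while CheckPieceMoves also reports attacks on the enemy king.
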(event EventBeginPlay
  (|CallParentFunction) ; This node is disabled and will not be called.\nDrag off pins to build functionality.
)

(event Collision|EventActorBeginOverlap
  (params (OtherActor :type Actor%20Object%20Reference))
  (|CallParentFunction OtherActor) ; This node is disabled and will not be called.\nDrag off pins to build functionality.
)

(event EventMovePiece
  (params (Piece :type BP%20Chess%20Pieces%20Object%20Reference) (Tile :type BP%20Tile%20Object%20Reference) (Number :type Integer) (Location :type Vector :default "0, 0, 0"))
  (bind _array_element (Utilities|Array|ForEachLoopwithBreak (Variables|Default|GetOut%20Actors) :!label _label)
    (:LoopBody
      (if (== (Variables|Default|GetCurrentTile) (Variables|/Game/MPChessTemplate/Blueprints/BP_Tile.BP_Tile_C|GetTileNumber _array_element))
        (Variables|/Game/MPChessTemplate/Blueprints/BP_Tile.BP_Tile_C|SetPiece _array_element 0)
        (Variables|Default|SetLastTile _array_element)
        (goto _label Break)))
    (:Completed
      (bind (_valid _take) (CallFunction|PieceMoveLogic Number (Variables|/Game/MPChessTemplate/Blueprints/BP_Tile.BP_Tile_C|GetOccupied Tile) (Variables|Default|GetFirstMove?) (and (Variables|/Game/MPChessTemplate/Blueprints/BP_Tile.BP_Tile_C|GetOccupied Tile) (!= (Variables|Default|GetTeam) (Variables|/Game/MPChessTemplate/Blueprints/BP_Tile.BP_Tile_C|GetTeam Tile))) (Variables|Default|GetKingChecked)))
      (if _valid
        (bind _output_get (Variables|Default|SetCurrentTile Number))
        (if _take
          (Default|DestroyPiece (Variables|/Game/MPChessTemplate/Blueprints/BP_Tile.BP_Tile_C|GetPiece Tile)))
        (CallFunction|SvrPieceMove _output_get Location Tile)
        (Utilities|FlowControl|Sequence
          (:then_0
            (Utilities|FlowControl|Delay 0.3)
            (CallFunction|KinginCheck?)
            (Default|CheckAllPieces (Variables|Default|GetAs%20Chess%20Game%20State)))
          (:then_1
            (Variables|Default|SetFirstMove? false)
            (Variables|/Game/MPChessTemplate/Blueprints/BP_Tile.BP_Tile_C|SetPiece Tile self)
            (Variables|/Game/MPChessTemplate/Blueprints/BP_Tile.BP_Tile_C|SetTeam Tile (Variables|Default|GetTeam))
            (Variables|/Game/MPChessTemplate/Blueprints/BP_Tile.BP_Tile_C|SetOccupied (Variables|Default|GetLastTile) false))
          (:then_2
            ;[1 1 1] PawnPromotion
            (switch int (Variables|Default|GetTeam)
              (:1
                (if (Utilities|Array|ContainsItem (Variables|Default|GetPromotionZoneP2) (Variables|Default|GetCurrentTile))
                  (Utilities|FlowControl|Delay 0.3 :!label _label_2)
                  (Default|PawnProZone (Variables|Default|GetAs%20Chess%20Game%20State) (Variables|Default|GetCurrentTile) (Variables|Default|GetTeam))
                  (CallFunction|DestroyPiece self)))
              (:2
                (if (Utilities|Array|ContainsItem (Variables|Default|GetPromotionZoneP1) (Variables|Default|GetCurrentTile))
                  (goto _label_2))))))))))

(fn ConstructionScript
  (|CallParentFunction))

(fn PieceMoveLogic
  (params (Tile :type Integer) (Occupied? :type Boolean) (FirstMove? :type Boolean) (EnemyOccupied? :type Boolean) (KingInCheck? :type Boolean))
  (bind _currenttile (Variables|Default|GetCurrentTile))
  (bind _currenttile_2 (Variables|Default|GetCurrentTile))
  (bind _currenttile_3 (Variables|Default|GetCurrentTile))
  (bind _currenttile_4 (Variables|Default|GetCurrentTile))
  (bind _inchecktiles (Variables|Default|GetInCheckTiles))
  (bind _returnvalue (Utilities|Array|ContainsItem _inchecktiles Tile))
  (bind _returnvalue_2 (- _currenttile Tile))
  (bind _returnvalue_3 (- Tile _currenttile_3))
  (bind _returnvalue_4 (- _currenttile_2 Tile))
  (bind _returnvalue_5 (- Tile _currenttile_4))
  ;[1 1 1] Black Or white??
  (switch int (Variables|Default|GetTeam)
    (:1
      (if FirstMove?
        ;[1 1 1] Forward 2 Tiles (First Move-Team White)
        (if (or (== _returnvalue_3 8) (== _returnvalue_3 16))
          (if Occupied? :!label _label
            _
            (elif KingInCheck?
              (if _returnvalue
                (return true false)
                (else
                  _))
              (else
                (return true false))))
          (else
            ;[1 1 1] Taking Pieces (Team White)
            (if (or (== _returnvalue_5 7) (== _returnvalue_5 9)) :!label _label_2
              (if EnemyOccupied?
                (if KingInCheck? :!label _label_3
                  (if _returnvalue
                    (return true true)
                    (else
                      _))
                  (else
                    (return true true)))))))
        (else
          ;[1 1 1] Forward 1 TIle (Team White)
          (if (== (- Tile _currenttile_4) 8)
            (goto _label)
            (else
              (goto _label_2))))))
    (:2
      (if FirstMove?
        ;[1 1 1] Forward 2 Tiles (First Move-Team Black
        (if (or (== _returnvalue_2 8) (== _returnvalue_2 16))
          (goto _label)
          (else
            _))
        (else
          ;[1 1 1] Froward 1 Tile (Team Black)
          (if (== (- (Variables|Default|GetCurrentTile) Tile) 8)
            (goto _label)
            (else
              _))))
      ;[1 1 1] Taking Piece (Team Black)
      (if (or (== _returnvalue_4 7) (== _returnvalue_4 9))
        (if EnemyOccupied?
          (goto _label_3)
          (else
            _)))))
  (return false false))

(fn CheckAvailable
  (params (Tiles :type Array%20of%20BP%20Tile%20Object%20References))
  (bind _currenttile (Variables|Default|GetCurrentTile))
  (bind _currenttile_2 (Variables|Default|GetCurrentTile))
  (bind _currenttile_3 (Variables|Default|GetCurrentTile))
  (bind _currenttile_4 (Variables|Default|GetCurrentTile))
  ;[1 1 1] Black Or white??
  (switch int (Variables|Default|GetTeam)
    (:1
      (for _array_element Tiles
        (if (Variables|Default|GetFirstMove?)
          ;[1 1 1] Check 2 tiles ahead (Team White First Move)
          (if (or (== (+ _currenttile_3 8) (Variables|/Game/MPChessTemplate/Blueprints/BP_Tile.BP_Tile_C|GetTileNumber _array_element)) (== (+ _currenttile_3 16) (Variables|/Game/MPChessTemplate/Blueprints/BP_Tile.BP_Tile_C|GetTileNumber _array_element)))
            (if (not (Variables|/Game/MPChessTemplate/Blueprints/BP_Tile.BP_Tile_C|GetOccupied _array_element))
              (Utilities|Array|AddUnique (LocalVariables|GetLocalAvailableTiles) (Variables|/Game/MPChessTemplate/Blueprints/BP_Tile.BP_Tile_C|GetTileNumber _array_element)))
            (else
              ;[1 1 1] Pawn Diagonal (Team White)
              (if (or (== (Variables|/Game/MPChessTemplate/Blueprints/BP_Tile.BP_Tile_C|GetTileNumber _array_element) (+ _currenttile_4 7)) (== (+ 9 _currenttile_4) (Variables|/Game/MPChessTemplate/Blueprints/BP_Tile.BP_Tile_C|GetTileNumber _array_element))) :!label _label
                (if (and (Variables|/Game/MPChessTemplate/Blueprints/BP_Tile.BP_Tile_C|GetOccupied _array_element) (== (Variables|/Game/MPChessTemplate/Blueprints/BP_Tile.BP_Tile_C|GetTeam _array_element) 2))
                  (Utilities|Array|AddUnique (LocalVariables|GetLocalAvailableTiles) (Variables|/Game/MPChessTemplate/Blueprints/BP_Tile.BP_Tile_C|GetTileNumber _array_element))))))
          (else
            ;[1 1 1] 1 tile forwat (Team White)
            (if (== (+ _currenttile_3 8) (Variables|/Game/MPChessTemplate/Blueprints/BP_Tile.BP_Tile_C|GetTileNumber _array_element))
              (if (not (Variables|/Game/MPChessTemplate/Blueprints/BP_Tile.BP_Tile_C|GetOccupied _array_element))
                (Utilities|Array|AddUnique (LocalVariables|GetLocalAvailableTiles) (Variables|/Game/MPChessTemplate/Blueprints/BP_Tile.BP_Tile_C|GetTileNumber _array_element)))
              (else
                (goto _label))))))
      (return (LocalVariables|GetLocalAvailableTiles)))
    (:2
      (for _array_element_2 Tiles
        (if (Variables|Default|GetFirstMove?)
          ;[1 1 1] Check 2 tiles ahead (Team Black First Move)
          (if (or (== (- _currenttile 8) (Variables|/Game/MPChessTemplate/Blueprints/BP_Tile.BP_Tile_C|GetTileNumber _array_element_2)) (== (- _currenttile 16) (Variables|/Game/MPChessTemplate/Blueprints/BP_Tile.BP_Tile_C|GetTileNumber _array_element_2)))
            (if (not (Variables|/Game/MPChessTemplate/Blueprints/BP_Tile.BP_Tile_C|GetOccupied _array_element_2))
              (Utilities|Array|AddUnique (LocalVariables|GetLocalAvailableTiles) (Variables|/Game/MPChessTemplate/Blueprints/BP_Tile.BP_Tile_C|GetTileNumber _array_element_2)))
            (else
              ;[1 1 1] Pawn Diagonal (Team Black)
              (if (or (== (Variables|/Game/MPChessTemplate/Blueprints/BP_Tile.BP_Tile_C|GetTileNumber _array_element_2) (- _currenttile_2 7)) (== (- _currenttile_2 9) (Variables|/Game/MPChessTemplate/Blueprints/BP_Tile.BP_Tile_C|GetTileNumber _array_element_2))) :!label _label_2
                (if (and (Variables|/Game/MPChessTemplate/Blueprints/BP_Tile.BP_Tile_C|GetOccupied _array_element_2) (== (Variables|/Game/MPChessTemplate/Blueprints/BP_Tile.BP_Tile_C|GetTeam _array_element_2) 1))
                  (Utilities|Array|AddUnique (LocalVariables|GetLocalAvailableTiles) (Variables|/Game/MPChessTemplate/Blueprints/BP_Tile.BP_Tile_C|GetTileNumber _array_element_2))))))
          (else
            ;[1 1 1] 1 tile forwat (Team Black)
            (if (== (- _currenttile 8) (Variables|/Game/MPChessTemplate/Blueprints/BP_Tile.BP_Tile_C|GetTileNumber _array_element_2))
              (if (not (Variables|/Game/MPChessTemplate/Blueprints/BP_Tile.BP_Tile_C|GetOccupied _array_element_2))
                (Utilities|Array|AddUnique (LocalVariables|GetLocalAvailableTiles) (Variables|/Game/MPChessTemplate/Blueprints/BP_Tile.BP_Tile_C|GetTileNumber _array_element_2)))
              (else
                (goto _label_2))))))
      (return (LocalVariables|GetLocalAvailableTiles)))))

(fn CheckPieceMoves
  (bind _currenttile (Variables|Default|GetCurrentTile))
  (bind _currenttile_2 (Variables|Default|GetCurrentTile))
  (bind _validmoves (Variables|Default|GetValidMoves))
  (bind _currenttile_3 (Variables|Default|GetCurrentTile))
  (bind _currenttile_4 (Variables|Default|GetCurrentTile))
  (bind _validmoves_2 (Variables|Default|GetValidMoves))
  (LocalVariables|SetKingCheck false)
  (LocalVariables|SetKingtilevar 0)
  (Utilities|Array|Clear (Variables|Default|GetInCheckTiles))
  ;[1 1 1] Black Or white??
  (switch int (Variables|Default|GetTeam)
    (:1
      (for _array_element (Variables|Default|GetOut%20Actors)
        (if (Variables|Default|GetFirstMove?)
          ;[1 1 1] Check 2 tiles ahead (Team White First Move)
          (if (or (== (+ _currenttile_3 8) (Variables|/Game/MPChessTemplate/Blueprints/BP_Tile.BP_Tile_C|GetTileNumber _array_element)) (== (+ _currenttile_3 16) (Variables|/Game/MPChessTemplate/Blueprints/BP_Tile.BP_Tile_C|GetTileNumber _array_element)))
            (if (Variables|/Game/MPChessTemplate/Blueprints/BP_Tile.BP_Tile_C|GetOccupied _array_element)
              _
              (else
                (Utilities|Array|AddUnique (Variables|Default|GetValidMoves) (Variables|/Game/MPChessTemplate/Blueprints/BP_Tile.BP_Tile_C|GetTileNumber _array_element)))))
          ;[1 1 1] Pawn Diagonal (Team White)
          (if (or (== (Variables|/Game/MPChessTemplate/Blueprints/BP_Tile.BP_Tile_C|GetTileNumber _array_element) (+ _currenttile_4 7)) (== (+ 9 _currenttile_4) (Variables|/Game/MPChessTemplate/Blueprints/BP_Tile.BP_Tile_C|GetTileNumber _array_element))) :!label _label
            (if (and (Variables|/Game/MPChessTemplate/Blueprints/BP_Tile.BP_Tile_C|GetOccupied _array_element) (== (Variables|/Game/MPChessTemplate/Blueprints/BP_Tile.BP_Tile_C|GetTeam _array_element) 2))
              (Utilities|Array|AddUnique (Variables|Default|GetValidMoves) (Variables|/Game/MPChessTemplate/Blueprints/BP_Tile.BP_Tile_C|GetTileNumber _array_element))
              ;[1 1 1] King Checks
              (if (Variables|/Game/MPChessTemplate/Blueprints/BP_Tile.BP_Tile_C|GetKing? _array_element)
                (Utilities|Array|AddUnique (Variables|Default|GetInCheckTiles) (Variables|Default|GetCurrentTile))
                (LocalVariables|SetKingtilevar _array_element)
                (LocalVariables|SetKingCheck true))))
          (else
            ;[1 1 1] 1 tile forwat (Team White)
            (if (== (+ _currenttile_3 8) (Variables|/Game/MPChessTemplate/Blueprints/BP_Tile.BP_Tile_C|GetTileNumber _array_element))
              (if (Variables|/Game/MPChessTemplate/Blueprints/BP_Tile.BP_Tile_C|GetOccupied _array_element)
                (goto _label)
                (else
                  (Utilities|Array|AddUnique (Variables|Default|GetValidMoves) (Variables|/Game/MPChessTemplate/Blueprints/BP_Tile.BP_Tile_C|GetTileNumber _array_element))))
              (else
                (goto _label))))))
      (if (LocalVariables|GetKingCheck)
        (return _validmoves_2 (Variables|Default|GetInCheckTiles) true (LocalVariables|GetKingtilevar) 0)
        (else
          (return _validmoves_2 0 false 0 0))))
    (:2
      (for _array_element_2 (Variables|Default|GetOut%20Actors)
        (if (Variables|Default|GetFirstMove?)
          ;[1 1 1] Check 2 tiles ahead (Team Black First Move)
          (if (or (== (- _currenttile 8) (Variables|/Game/MPChessTemplate/Blueprints/BP_Tile.BP_Tile_C|GetTileNumber _array_element_2)) (== (- _currenttile 16) (Variables|/Game/MPChessTemplate/Blueprints/BP_Tile.BP_Tile_C|GetTileNumber _array_element_2)))
            (if (Variables|/Game/MPChessTemplate/Blueprints/BP_Tile.BP_Tile_C|GetOccupied _array_element_2)
              _
              (else
                (Utilities|Array|AddUnique (Variables|Default|GetValidMoves) (Variables|/Game/MPChessTemplate/Blueprints/BP_Tile.BP_Tile_C|GetTileNumber _array_element_2)))))
          ;[1 1 1] Pawn Diagonal (Team Black)
          (if (or (== (Variables|/Game/MPChessTemplate/Blueprints/BP_Tile.BP_Tile_C|GetTileNumber _array_element_2) (- _currenttile_2 7)) (== (- _currenttile_2 9) (Variables|/Game/MPChessTemplate/Blueprints/BP_Tile.BP_Tile_C|GetTileNumber _array_element_2))) :!label _label_2
            (if (and (Variables|/Game/MPChessTemplate/Blueprints/BP_Tile.BP_Tile_C|GetOccupied _array_element_2) (== (Variables|/Game/MPChessTemplate/Blueprints/BP_Tile.BP_Tile_C|GetTeam _array_element_2) 1))
              (Utilities|Array|AddUnique (Variables|Default|GetValidMoves) (Variables|/Game/MPChessTemplate/Blueprints/BP_Tile.BP_Tile_C|GetTileNumber _array_element_2))
              ;[1 1 1] King Checks
              (if (Variables|/Game/MPChessTemplate/Blueprints/BP_Tile.BP_Tile_C|GetKing? _array_element_2)
                (Utilities|Array|AddUnique (Variables|Default|GetInCheckTiles) (Variables|Default|GetCurrentTile))
                (LocalVariables|SetKingtilevar _array_element_2)
                (LocalVariables|SetKingCheck true))))
          (else
            ;[1 1 1] 1 tile forwat (Team Black)
            (if (== (- _currenttile 8) (Variables|/Game/MPChessTemplate/Blueprints/BP_Tile.BP_Tile_C|GetTileNumber _array_element_2))
              (if (Variables|/Game/MPChessTemplate/Blueprints/BP_Tile.BP_Tile_C|GetOccupied _array_element_2)
                (goto _label_2)
                (else
                  (Utilities|Array|AddUnique (Variables|Default|GetValidMoves) (Variables|/Game/MPChessTemplate/Blueprints/BP_Tile.BP_Tile_C|GetTileNumber _array_element_2))))
              (else
                (goto _label_2))))))
      (if (LocalVariables|GetKingCheck)
        (return _validmoves (Variables|Default|GetInCheckTiles) true (LocalVariables|GetKingtilevar) 0)
        (else
          (return _validmoves 0 false 0 0))))))